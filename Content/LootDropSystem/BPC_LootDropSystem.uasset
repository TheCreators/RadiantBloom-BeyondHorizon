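; Loot drop component that spawns a random number of items at its owner's location when DropLoot is called.
; ChooseDrop makes a weighted random pick from PossibleDrop by relative weight, returning a data table row handle that resolves to the item class to spawn.
; Spawned actors implementing BPI_LootDropMesh expose their mesh, which receives a random velocity impulse within a wide upward cone to scatter the loot.
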(event `Drop Loot`
  (for _ (range (`KismetMathLibrary.RandomIntegerInRange` (`self.Min Drop Amount`) (`self.Max Drop Amount`)))
    (bind (_item _success) (`self.Choose Drop`))
    (if _success
      (bind _returnvalue (`|GetDataTableRow` (break `DataTableRowHandle` _item) (`.RowName` (break `DataTableRowHandle` _item)))
        (:`then`
          (bind _returnvalue_2 (`|SpawnActorFromClass` (`.ItemClass_10_B2A021554022D9D4B1CF23B92DCE0FE0` (break `/Game/Inventory/S_Item` _returnvalue)) (`KismetMathLibrary.MakeTransform` (`Actor.K2_GetActorLocation` (`self.GetOwner`))) "Undefined" "MultiplyWithRoot" null null))
          (if (`KismetSystemLibrary.DoesImplementInterface` _returnvalue_2 "/Game/LootDropSystem/BPI_LootDropMesh.BPI_LootDropMesh_C")
            (bind _mesh (message `/Game/LootDropSystem/BPI_LootDropMesh.Get Mesh` _returnvalue_2))
            (`PrimitiveComponent.AddImpulse` _mesh (* (`KismetMathLibrary.RandomUnitVectorInConeInDegrees` (0.0 0.0 1.0) 120.0) (`KismetMathLibrary.RandomFloatInRange` 200.0 500.0)) "None" true)
            (`KismetSystemLibrary.PrintString` "Hello")))))))

(fn `Choose Drop`
  (returns (Item :type "DataTableRowHandle Structure") (Success :type Boolean))
  (locals (`Local Weight Sum` :type Integer) (`Local Random Choice` :type Integer))
  (if (`KismetArrayLibrary.Array_IsNotEmpty` (`self.Possible Drop`))
    (for _array_element (`self.Possible Drop`)
      (set `local.Local Weight Sum` (+ (`.RelativeDropWeight_15_D90E90314761811D4920C181830BFFFB` (break `/Game/LootDropSystem/S_LootDrop` _array_element)) (`local.Local Weight Sum`))))
    (set `local.Local Random Choice` (`KismetMathLibrary.RandomIntegerInRange` 0 (`local.Local Weight Sum`)))
    (for _array_element_2 (`self.Possible Drop`)
      (bind _output_get (set `local.Local Random Choice` (- (`local.Local Random Choice`) (`.RelativeDropWeight_15_D90E90314761811D4920C181830BFFFB` (break `/Game/LootDropSystem/S_LootDrop` _array_element_2)))))
      (if (<= _output_get 0)
        (return (break `/Game/LootDropSystem/S_LootDrop` _array_element_2) true)))
    (`KismetSystemLibrary.PrintString` "LOOP DROP ERROR!!!" true true (struct :`R` 1.0 :`G` 0.025124 :`A` 1.0) 5.0)
    (return (struct) false)
    (else
      (return (struct) false))))