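; BPC_LevelingSystem is a component that tracks player XP and level and broadcasts XP, level-up and level-init events.
; AddXP recursively carries overflow through multiple level-ups, with each new threshold growing exponentially from FirstLevelXP by NextLevelXPRatio.
; AddRelativeXP grants XP as a fraction of the current threshold.
; It requests a load from the GameInstance on BeginPlay, broadcasts initial state a tick later, and saves progress to the SaveGame's leveling struct.
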(event `self.ReceiveBeginPlay`
  ;[0.8984 0 1] Request Load
  (message `/Game/Save/BPI_Persistence.RequestLoad` (`GameplayStatics.GetGameInstance`) self)
  (`KismetSystemLibrary.DelayUntilNextTick`)
  (`self.OnXPChanged` (`self.XP`) (`self.LevelUpXP`))
  (`self.OnLevelInit` (`self.Level`)))

(event `/Game/Save/BPI_Saveable.SaveData`
  (params (SaveGameRef :type "/Game/Save/BP_SaveGame Object Reference"))
  ;[0 1 0.9297] Save
  (set `/Game/Save/BP_SaveGame.PlayerLevelingSaveData` (make `/Game/Save/Structures/S_PlayerLevelingSaveData` (`self.XP`) (`self.Level`) (`self.LevelUpXP`)) SaveGameRef))

(event `/Game/Save/BPI_Saveable.LoadData`
  (params (SaveGameRef :type "/Game/Save/BP_SaveGame Object Reference"))
  (bind (_xp _level _levelupxp) (break `/Game/Save/Structures/S_PlayerLevelingSaveData` (`/Game/Save/BP_SaveGame.PlayerLevelingSaveData` SaveGameRef)))
  ;[0 1 0.9297] Save
  (set `self.XP` _xp)
  (set `self.Level` _level)
  (set `self.LevelUpXP` _levelupxp))

(fn `AddRelativeXP`
  (params (`Relative Amount` :type "Float (double-precision)" :default 0.1))
  (`self.AddXP` (`self.GetAbsoluteXP` `Relative Amount`)))

(fn `AddXP`
  (params (Amount :type Integer64))
  (locals (Local_TotalXP :type Integer64) (Local_XPAfterLevelUp :type Integer64))
  (set `local.Local_TotalXP` (+ (`local.Amount`) (`self.XP`)))
  (if (>= (`local.Local_TotalXP`) (`self.LevelUpXP`))
    (set `local.Local_XPAfterLevelUp` (- (`local.Local_TotalXP`) (`self.LevelUpXP`)))
    (`self.LevelUp`)
    (set `self.XP` 0)
    (`self.AddXP` (`local.Local_XPAfterLevelUp`))
    (else
      (set `self.XP` (`local.Local_TotalXP`))
      (`self.OnXPChanged` (`self.XP`) (`self.LevelUpXP`)))))

(fn `GetAbsoluteXP`
  (params (RelativeXP :type "Float (double-precision)"))
  (returns (AbsoluteXP :type Integer64))
  (return (`KismetMathLibrary.Conv_DoubleToInt64` (* (`KismetMathLibrary.Conv_Int64ToDouble` (`self.LevelUpXP`)) (`local.RelativeXP`)))))

(fn `LevelUp`
  (`/Engine/EditorBlueprintResources/StandardMacros.IncrementInt` (`self.Level`)
    (:`  `
      (`self.OnLevelUp` (`self.Level`))
      (set `self.LevelUpXP` (`KismetMathLibrary.Conv_DoubleToInt64` (* (`KismetMathLibrary.Conv_Int64ToDouble` (`self.FirstLevelXP`)) (`KismetMathLibrary.MultiplyMultiply_FloatFloat` (`self.NextLevelXPRatio`) (`KismetMathLibrary.Conv_IntToDouble` (`/Game/UlimateBlueprintPack/System/Blueprints/UBPP_FunctionLibrary.Minus One (Int)` (`self.Level`)))))))
      (`self.OnXPChanged` (`self.XP`) (`self.LevelUpXP`)))))