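; Stores named character customization profiles for the modular medieval NPC character editor in a CustomizationData array.
; Saving snapshots a character's parts, hat visibility, tint settings and colors into a struct, overwrites entries with the same profile name, then appends the snapshot after the loop.
; Loading, listing and deleting scan the array by name, with load returning a success flag, and a separate function clears all profiles.
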(fn `CreateCustomizationData`
  (params (ProfileName :type String) (BP_Character :type "/Game/ModularMedievalNPC/Character/Blueprints/BP_CustomizableCharacter Object Reference"))
  (returns (ReturnValue :type "/Game/ModularMedievalNPC/CharacterEditor/Blueprints/SCustomizationData Structure"))
  (return (make `/Game/ModularMedievalNPC/CharacterEditor/Blueprints/SCustomizationData` ProfileName (`/Game/ModularMedievalNPC/Character/Blueprints/BP_CustomizableCharacter.bHideHat` BP_Character) (`/Game/ModularMedievalNPC/Character/Blueprints/BP_CustomizableCharacter.Hat` BP_Character) (`/Game/ModularMedievalNPC/Character/Blueprints/BP_CustomizableCharacter.Hair` BP_Character) (`/Game/ModularMedievalNPC/Character/Blueprints/BP_CustomizableCharacter.Head` BP_Character) (`/Game/ModularMedievalNPC/Character/Blueprints/BP_CustomizableCharacter.Chest` BP_Character) (`/Game/ModularMedievalNPC/Character/Blueprints/BP_CustomizableCharacter.Arm` BP_Character) (`/Game/ModularMedievalNPC/Character/Blueprints/BP_CustomizableCharacter.Leg` BP_Character) (`/Game/ModularMedievalNPC/Character/Blueprints/BP_CustomizableCharacter.RightHand` BP_Character) (`/Game/ModularMedievalNPC/Character/Blueprints/BP_CustomizableCharacter.LeftHand` BP_Character) (`/Game/ModularMedievalNPC/Character/Blueprints/BP_CustomizableCharacter.TintMode` BP_Character) (`/Game/ModularMedievalNPC/Character/Blueprints/BP_CustomizableCharacter.SK_Parts (Equipment)` BP_Character) (`/Game/ModularMedievalNPC/Character/Blueprints/BP_CustomizableCharacter.SK_Parts (Hair)` BP_Character) (`/Game/ModularMedievalNPC/Character/Blueprints/BP_CustomizableCharacter.SM_Parts (Attachments)` BP_Character) (`/Game/ModularMedievalNPC/Character/Blueprints/BP_CustomizableCharacter.Skin` BP_Character) (`/Game/ModularMedievalNPC/Character/Blueprints/BP_CustomizableCharacter.Primary` BP_Character) (`/Game/ModularMedievalNPC/Character/Blueprints/BP_CustomizableCharacter.Details1` BP_Character) (`/Game/ModularMedievalNPC/Character/Blueprints/BP_CustomizableCharacter.Details2` BP_Character) (`/Game/ModularMedievalNPC/Character/Blueprints/BP_CustomizableCharacter.Details3 / Skin` BP_Character))))

(fn `DeleteAllCustomizationData`
  (`KismetArrayLibrary.Array_Clear` (`self.CustomizationData`)))

(fn `DeleteCustomizationData`
  (params (ProfileName :type String))
  (for _array_element (`self.CustomizationData`)
    (if (`KismetStringLibrary.EqualEqual_StrStr` ProfileName (`.ProfileName_33_1E9250D841658025EF1AC4A978AEA6BC` (break `/Game/ModularMedievalNPC/CharacterEditor/Blueprints/SCustomizationData` _array_element)))
      (`KismetArrayLibrary.Array_RemoveItem` (`self.CustomizationData`) _array_element))))

(fn `GetCustomizationDataByProfileName`
  (params (ProfileName :type String))
  (returns (ReturnValue :type "/Game/ModularMedievalNPC/CharacterEditor/Blueprints/SCustomizationData Structure") (Index :type Integer))
  (for (_array_element _array_index) (`self.CustomizationData`)
    (if (`KismetStringLibrary.EqualEqual_StrStr` ProfileName (`.ProfileName_33_1E9250D841658025EF1AC4A978AEA6BC` (break `/Game/ModularMedievalNPC/CharacterEditor/Blueprints/SCustomizationData` _array_element)))
      (return _array_element _array_index)))
  (return (struct) -1))

(fn `GetProfileNames`
  (returns (ReturnValue :type "Array of String"))
  (locals (ProfileNames :type "Array of String"))
  (for _array_element (`self.CustomizationData`)
    (`KismetArrayLibrary.Array_Add` (`local.ProfileNames`) (`.ProfileName_33_1E9250D841658025EF1AC4A978AEA6BC` (break `/Game/ModularMedievalNPC/CharacterEditor/Blueprints/SCustomizationData` _array_element))))
  (return (`local.ProfileNames`)))

(fn `LoadCustomizationData`
  (params (ProfileName :type String))
  (returns (ReturnValue :type Boolean) (CustomizationData :type "/Game/ModularMedievalNPC/CharacterEditor/Blueprints/SCustomizationData Structure"))
  (bind (_returnvalue _index) (`self.GetCustomizationDataByProfileName` ProfileName))
  (if (!= _index -1)
    (return true _returnvalue)
    (else
      (return false))))

(fn `SaveCustomizationData`
  (params (ProfileName :type String) (BP_Character :type "/Game/ModularMedievalNPC/Character/Blueprints/BP_CustomizableCharacter Object Reference"))
  (for (_array_element _array_index) (`self.CustomizationData`)
    ;[0 0 0] Update and save an existing save data matching the Profile Name
    (if (`KismetStringLibrary.EqualEqual_StrStr` (`.ProfileName_33_1E9250D841658025EF1AC4A978AEA6BC` (break `/Game/ModularMedievalNPC/CharacterEditor/Blueprints/SCustomizationData` _array_element)) ProfileName)
      (`KismetArrayLibrary.Array_Set` (`self.CustomizationData`) _array_index (`self.CreateCustomizationData` ProfileName BP_Character))))
  ;[0 0 0] Save new data with Profile Name
  (`KismetArrayLibrary.Array_Add` (`self.CustomizationData`) (`self.CreateCustomizationData` ProfileName BP_Character)))