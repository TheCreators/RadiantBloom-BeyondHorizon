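; BP_SpawnProxy is a placement indicator in the character editor that marks where a new customized NPC will spawn.
; Each Tick it line traces from the deprojected mouse cursor on the Visibility channel and moves itself to the hit location.
; Its Spawn event creates a BP_PlayerCharacter there, raised by the capsule half-height and yawed opposite the control rotation, applies the CustomizationData, then destroys the proxy.
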(event `self.ReceiveTick`
  (params (DeltaSeconds :type "Float (single-precision)"))
  (bind (_worldlocation _worlddirection) (`PlayerController.DeprojectMousePositionToWorld` (`GameplayStatics.GetPlayerController` 0)))
  ;[0 0 0] Set Actor Location to mouse cursor on ground, as an indicator for spawn location
  (bind _outhit (`KismetSystemLibrary.LineTraceSingle` _worldlocation (+ _worldlocation (* _worlddirection 2000.0)) "TraceTypeQuery1" true))
  (`self.K2_SetActorLocation` (`.Location` (`GameplayStatics.BreakHitResult` _outhit))))

(event `Spawn`
  (bind (_returnvalue_roll _returnvalue_pitch _returnvalue_yaw) (`KismetMathLibrary.BreakRotator` (`Controller.GetControlRotation` (`GameplayStatics.GetPlayerController` 0))))
  ;[0 0 0] Spawn a new Character at last Hit Location as an NPC, apply Customization and destroy this SpawnProxy
  (bind _returnvalue (`|SpawnActorFromClass` "/Game/ModularMedievalNPC/Character/Blueprints/BP_PlayerCharacter.BP_PlayerCharacter_C" (`KismetMathLibrary.MakeTransform` (+ (`.Location` (`GameplayStatics.BreakHitResult` (stale `self.ReceiveTick` _outhit))) (0.0 0.0 96.0)) (`KismetMathLibrary.MakeRotator` 0.0 0.0 (+ _returnvalue_yaw 180.0))) "Undefined" "OverrideRootScale" null null))
  (`/Game/ModularMedievalNPC/Character/Blueprints/BP_PlayerCharacter.ApplyCustomizationData` _returnvalue (`self.CustomizationData`))
  (`self.K2_DestroyActor`))

(fn `UserConstructionScript`)