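; Light rig for the modular NPC character editor, with key, back, rim and spot lights that start dark.
; Construction caches each light's intensity, then zeroes them unless DebugLightIntensity is set; BeginPlay always zeroes them.
; UpdateLights scales all four from zero to their cached intensity by an Alpha and shows the static mesh only above zero.
; Tick pins the FixedRotation component to zero world rotation.
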(event `self.ReceiveBeginPlay`
  (`self.UpdateLights` 0.0))

(event `self.ReceiveTick`
  (params (DeltaSeconds :type "Float (single-precision)"))
  (`SceneComponent.K2_SetWorldRotation` :`self` (`self.FixedRotation`)))

(fn `UpdateLights`
  (params (Alpha :type "Float (double-precision)"))
  (`LightComponent.SetIntensity` (`self.KeyLight`) (`KismetMathLibrary.Lerp` 0.0 (`self.KeyLightIntensity`) Alpha))
  (`LightComponent.SetIntensity` (`self.BackLight`) (`KismetMathLibrary.Lerp` 0.0 (`self.BackLightIntensity`) Alpha))
  (`LightComponent.SetIntensity` (`self.RimLight`) (`KismetMathLibrary.Lerp` 0.0 (`self.RimLightIntensity`) Alpha))
  (`LightComponent.SetIntensity` (`self.SpotLight`) (`KismetMathLibrary.Lerp` 0.0 (`self.SpotLight_intensity`) Alpha))
  (`SceneComponent.SetVisibility` (`self.StaticMesh`) (> Alpha 0.0) false))

(fn `UserConstructionScript`
  (set `self.KeyLightIntensity` (`LightComponentBase.Intensity` (`self.KeyLight`)))
  (set `self.BackLightIntensity` (`LightComponentBase.Intensity` (`self.BackLight`)))
  (set `self.RimLightIntensity` (`LightComponentBase.Intensity` (`self.RimLight`)))
  (set `self.SpotLight_intensity` (`LightComponentBase.Intensity` (`self.SpotLight`)))
  (if (not (`self.DebugLightIntensity`))
    (`self.UpdateLights` 0.0)))