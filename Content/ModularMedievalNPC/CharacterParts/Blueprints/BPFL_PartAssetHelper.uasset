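; Function library for modular medieval NPCs that finds part assets and picks default or random character outfits.
; Asset Registry queries by class, optionally filtered by gameplay tags, load the candidates for each slot.
; Defaults take the first body part found; random picks also fill both hands, with an empty option.
; Helpers map slots to classes, convert morph flags to weights and insertion-sort parts by display name, comparing character codes.
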(fn `GetDefaultPartAssets`
  (returns (Hat :type "/Game/ModularMedievalNPC/CharacterParts/Blueprints/BP_PartAsset_SK_Hat Object Reference") (Hair :type "/Game/ModularMedievalNPC/CharacterParts/Blueprints/BP_PartAsset_SK_Hair Object Reference") (Head :type "/Game/ModularMedievalNPC/CharacterParts/Blueprints/BP_PartAsset_SK_Head Object Reference") (Chest :type "/Game/ModularMedievalNPC/CharacterParts/Blueprints/BP_PartAsset_SK_Chest Object Reference") (Arm :type "/Game/ModularMedievalNPC/CharacterParts/Blueprints/BP_PartAsset_SK_Arm Object Reference") (Leg :type "/Game/ModularMedievalNPC/CharacterParts/Blueprints/BP_PartAsset_SK_Leg Object Reference") (RightHand :type "/Game/ModularMedievalNPC/CharacterParts/Blueprints/BP_PartAsset_SM_HandItem Object Reference") (LeftHand :type "/Game/ModularMedievalNPC/CharacterParts/Blueprints/BP_PartAsset_SM_HandItem Object Reference"))
  (bind ___worldcontext (`local.__WorldContext`))
  (`|ExecutionSequence`
    (:`then_0`
      (bind (_returnvalue _partassets) (`self.GetPartAssetsFromAssetRegistry` "/Game/ModularMedievalNPC/CharacterParts/Blueprints/BP_PartAsset_SK_Hat.BP_PartAsset_SK_Hat_C" false ___worldcontext)) ; Hat
      (if _returnvalue
        (bind _asbp_part_asset_sk_hat (cast `/Game/ModularMedievalNPC/CharacterParts/Blueprints/BP_PartAsset_SK_Hat` (`/Game/ModularMedievalNPC/CharacterParts/Blueprints/BPML_PartAssetHelper.GetFirstArrayElement` _partassets)))
        (bind _get (`/Game/ModularMedievalNPC/CharacterParts/Blueprints/BPML_PartAssetHelper.TempVariable` _asbp_part_asset_sk_hat))))
    (:`then_1`
      (bind (_returnvalue_2 _partassets_2) (`self.GetPartAssetsFromAssetRegistry` "/Game/ModularMedievalNPC/CharacterParts/Blueprints/BP_PartAsset_SK_Hair.BP_PartAsset_SK_Hair_C" false ___worldcontext)) ; Hair
      (if _returnvalue_2
        (bind _asbp_part_asset_sk_hair (cast `/Game/ModularMedievalNPC/CharacterParts/Blueprints/BP_PartAsset_SK_Hair` (`/Game/ModularMedievalNPC/CharacterParts/Blueprints/BPML_PartAssetHelper.GetFirstArrayElement` _partassets_2)))
        (bind _get_2 (`/Game/ModularMedievalNPC/CharacterParts/Blueprints/BPML_PartAssetHelper.TempVariable` _asbp_part_asset_sk_hair))))
    (:`then_2`
      (bind (_returnvalue_3 _partassets_3) (`self.GetPartAssetsFromAssetRegistry` "/Game/ModularMedievalNPC/CharacterParts/Blueprints/BP_PartAsset_SK_Head.BP_PartAsset_SK_Head_C" false ___worldcontext)) ; Head
      (if _returnvalue_3
        (bind _asbp_part_asset_sk_head (cast `/Game/ModularMedievalNPC/CharacterParts/Blueprints/BP_PartAsset_SK_Head` (`/Game/ModularMedievalNPC/CharacterParts/Blueprints/BPML_PartAssetHelper.GetFirstArrayElement` _partassets_3)))
        (bind _get_3 (`/Game/ModularMedievalNPC/CharacterParts/Blueprints/BPML_PartAssetHelper.TempVariable` _asbp_part_asset_sk_head))))
    (:`then_3`
      (bind (_returnvalue_4 _partassets_4) (`self.GetPartAssetsFromAssetRegistry` "/Game/ModularMedievalNPC/CharacterParts/Blueprints/BP_PartAsset_SK_Chest.BP_PartAsset_SK_Chest_C" false ___worldcontext)) ; Chest
      (if _returnvalue_4
        (bind _asbp_part_asset_sk_chest (cast `/Game/ModularMedievalNPC/CharacterParts/Blueprints/BP_PartAsset_SK_Chest` (`/Game/ModularMedievalNPC/CharacterParts/Blueprints/BPML_PartAssetHelper.GetFirstArrayElement` _partassets_4)))
        (bind _get_4 (`/Game/ModularMedievalNPC/CharacterParts/Blueprints/BPML_PartAssetHelper.TempVariable` _asbp_part_asset_sk_chest))))
    (:`then_4`
      (bind (_returnvalue_5 _partassets_5) (`self.GetPartAssetsFromAssetRegistry` "/Game/ModularMedievalNPC/CharacterParts/Blueprints/BP_PartAsset_SK_Arm.BP_PartAsset_SK_Arm_C" false ___worldcontext)) ; Arm
      (if _returnvalue_5
        (bind _asbp_part_asset_sk_arm (cast `/Game/ModularMedievalNPC/CharacterParts/Blueprints/BP_PartAsset_SK_Arm` (`/Game/ModularMedievalNPC/CharacterParts/Blueprints/BPML_PartAssetHelper.GetFirstArrayElement` _partassets_5)))
        (bind _get_5 (`/Game/ModularMedievalNPC/CharacterParts/Blueprints/BPML_PartAssetHelper.TempVariable` _asbp_part_asset_sk_arm))))
    (:`then_5`
      (bind (_returnvalue_6 _partassets_6) (`self.GetPartAssetsFromAssetRegistry` "/Game/ModularMedievalNPC/CharacterParts/Blueprints/BP_PartAsset_SK_Leg.BP_PartAsset_SK_Leg_C" false ___worldcontext)) ; Leg
      (if _returnvalue_6
        (bind _asbp_part_asset_sk_leg (cast `/Game/ModularMedievalNPC/CharacterParts/Blueprints/BP_PartAsset_SK_Leg` (`/Game/ModularMedievalNPC/CharacterParts/Blueprints/BPML_PartAssetHelper.GetFirstArrayElement` _partassets_6)))
        (bind _get_6 (`/Game/ModularMedievalNPC/CharacterParts/Blueprints/BPML_PartAssetHelper.TempVariable` _asbp_part_asset_sk_leg))))
    (:`then_6`
      (return _get _get_2 _get_3 _get_4 _get_5 _get_6 null null))))

(fn `GetDefaultPartAssetsByPartTags`
  (params (PartAssetFilter :type "GameplayTagContainer Structure") (ExcludeEmptyPartTags :type Boolean))
  (returns (Hat :type "/Game/ModularMedievalNPC/CharacterParts/Blueprints/BP_PartAsset_SK_Hat Object Reference") (Hair :type "/Game/ModularMedievalNPC/CharacterParts/Blueprints/BP_PartAsset_SK_Hair Object Reference") (Head :type "/Game/ModularMedievalNPC/CharacterParts/Blueprints/BP_PartAsset_SK_Head Object Reference") (Chest :type "/Game/ModularMedievalNPC/CharacterParts/Blueprints/BP_PartAsset_SK_Chest Object Reference") (Arm :type "/Game/ModularMedievalNPC/CharacterParts/Blueprints/BP_PartAsset_SK_Arm Object Reference") (Leg :type "/Game/ModularMedievalNPC/CharacterParts/Blueprints/BP_PartAsset_SK_Leg Object Reference") (RightHand :type "/Game/ModularMedievalNPC/CharacterParts/Blueprints/BP_PartAsset_SM_HandItem Object Reference") (LeftHand :type "/Game/ModularMedievalNPC/CharacterParts/Blueprints/BP_PartAsset_SM_HandItem Object Reference"))
  (bind ___worldcontext (`local.__WorldContext`))
  (`|ExecutionSequence`
    (:`then_0`
      (bind (_returnvalue _partassets) (`self.GetPartAssetsFromAssetRegistryByPartTags` "/Game/ModularMedievalNPC/CharacterParts/Blueprints/BP_PartAsset_SK_Hat.BP_PartAsset_SK_Hat_C" PartAssetFilter ExcludeEmptyPartTags false ___worldcontext)) ; Hat
      (if _returnvalue
        (bind _asbp_part_asset_sk_hat (cast `/Game/ModularMedievalNPC/CharacterParts/Blueprints/BP_PartAsset_SK_Hat` (`/Game/ModularMedievalNPC/CharacterParts/Blueprints/BPML_PartAssetHelper.GetFirstArrayElement` _partassets)))
        (bind _get (`/Game/ModularMedievalNPC/CharacterParts/Blueprints/BPML_PartAssetHelper.TempVariable` _asbp_part_asset_sk_hat))))
    (:`then_1`
      (bind (_returnvalue_2 _partassets_2) (`self.GetPartAssetsFromAssetRegistryByPartTags` "/Game/ModularMedievalNPC/CharacterParts/Blueprints/BP_PartAsset_SK_Hair.BP_PartAsset_SK_Hair_C" PartAssetFilter ExcludeEmptyPartTags false ___worldcontext)) ; Hair
      (if _returnvalue_2
        (bind _asbp_part_asset_sk_hair (cast `/Game/ModularMedievalNPC/CharacterParts/Blueprints/BP_PartAsset_SK_Hair` (`/Game/ModularMedievalNPC/CharacterParts/Blueprints/BPML_PartAssetHelper.GetFirstArrayElement` _partassets_2)))
        (bind _get_2 (`/Game/ModularMedievalNPC/CharacterParts/Blueprints/BPML_PartAssetHelper.TempVariable` _asbp_part_asset_sk_hair))))
    (:`then_2`
      (bind (_returnvalue_3 _partassets_3) (`self.GetPartAssetsFromAssetRegistryByPartTags` "/Game/ModularMedievalNPC/CharacterParts/Blueprints/BP_PartAsset_SK_Head.BP_PartAsset_SK_Head_C" PartAssetFilter ExcludeEmptyPartTags false ___worldcontext)) ; Head
      (if _returnvalue_3
        (bind _asbp_part_asset_sk_head (cast `/Game/ModularMedievalNPC/CharacterParts/Blueprints/BP_PartAsset_SK_Head` (`/Game/ModularMedievalNPC/CharacterParts/Blueprints/BPML_PartAssetHelper.GetFirstArrayElement` _partassets_3)))
        (bind _get_3 (`/Game/ModularMedievalNPC/CharacterParts/Blueprints/BPML_PartAssetHelper.TempVariable` _asbp_part_asset_sk_head))))
    (:`then_3`
      (bind (_returnvalue_4 _partassets_4) (`self.GetPartAssetsFromAssetRegistryByPartTags` "/Game/ModularMedievalNPC/CharacterParts/Blueprints/BP_PartAsset_SK_Chest.BP_PartAsset_SK_Chest_C" PartAssetFilter ExcludeEmptyPartTags false ___worldcontext)) ; Chest
      (if _returnvalue_4
        (bind _asbp_part_asset_sk_chest (cast `/Game/ModularMedievalNPC/CharacterParts/Blueprints/BP_PartAsset_SK_Chest` (`/Game/ModularMedievalNPC/CharacterParts/Blueprints/BPML_PartAssetHelper.GetFirstArrayElement` _partassets_4)))
        (bind _get_4 (`/Game/ModularMedievalNPC/CharacterParts/Blueprints/BPML_PartAssetHelper.TempVariable` _asbp_part_asset_sk_chest))))
    (:`then_4`
      (bind (_returnvalue_5 _partassets_5) (`self.GetPartAssetsFromAssetRegistryByPartTags` "/Game/ModularMedievalNPC/CharacterParts/Blueprints/BP_PartAsset_SK_Arm.BP_PartAsset_SK_Arm_C" PartAssetFilter ExcludeEmptyPartTags false ___worldcontext)) ; Arm
      (if _returnvalue_5
        (bind _asbp_part_asset_sk_arm (cast `/Game/ModularMedievalNPC/CharacterParts/Blueprints/BP_PartAsset_SK_Arm` (`/Game/ModularMedievalNPC/CharacterParts/Blueprints/BPML_PartAssetHelper.GetFirstArrayElement` _partassets_5)))
        (bind _get_5 (`/Game/ModularMedievalNPC/CharacterParts/Blueprints/BPML_PartAssetHelper.TempVariable` _asbp_part_asset_sk_arm))))
    (:`then_5`
      (bind (_returnvalue_6 _partassets_6) (`self.GetPartAssetsFromAssetRegistryByPartTags` "/Game/ModularMedievalNPC/CharacterParts/Blueprints/BP_PartAsset_SK_Leg.BP_PartAsset_SK_Leg_C" PartAssetFilter ExcludeEmptyPartTags false ___worldcontext)) ; Leg
      (if _returnvalue_6
        (bind _asbp_part_asset_sk_leg (cast `/Game/ModularMedievalNPC/CharacterParts/Blueprints/BP_PartAsset_SK_Leg` (`/Game/ModularMedievalNPC/CharacterParts/Blueprints/BPML_PartAssetHelper.GetFirstArrayElement` _partassets_6)))
        (bind _get_6 (`/Game/ModularMedievalNPC/CharacterParts/Blueprints/BPML_PartAssetHelper.TempVariable` _asbp_part_asset_sk_leg))))
    (:`then_6`
      (return _get _get_2 _get_3 _get_4 _get_5 _get_6 null null))))

(fn `GetMorphTargetValue`
  (params (CanMorph :type Boolean))
  (returns (ReturnValue :type "Float (double-precision)"))
  (return (`KismetMathLibrary.SelectFloat` 1.0 0.0 CanMorph)))

(fn `GetPartAssetClass`
  (params (Slot :type "/Game/ModularMedievalNPC/CharacterParts/Blueprints/ESlot Enum" :default "NewEnumerator3"))
  (returns (ReturnValue :type "/Game/ModularMedievalNPC/CharacterParts/Blueprints/BP_PartAsset Class Reference"))
  (return (select `/Game/ModularMedievalNPC/CharacterParts/Blueprints/ESlot` Slot :`NewEnumerator3` "/Game/ModularMedievalNPC/CharacterParts/Blueprints/BP_PartAsset_SK_Hat.BP_PartAsset_SK_Hat_C" :`NewEnumerator7` "/Game/ModularMedievalNPC/CharacterParts/Blueprints/BP_PartAsset_SK_Hair.BP_PartAsset_SK_Hair_C" :`NewEnumerator6` "/Game/ModularMedievalNPC/CharacterParts/Blueprints/BP_PartAsset_SK_Head.BP_PartAsset_SK_Head_C" :`NewEnumerator0` "/Game/ModularMedievalNPC/CharacterParts/Blueprints/BP_PartAsset_SK_Chest.BP_PartAsset_SK_Chest_C" :`NewEnumerator1` "/Game/ModularMedievalNPC/CharacterParts/Blueprints/BP_PartAsset_SK_Arm.BP_PartAsset_SK_Arm_C" :`NewEnumerator2` "/Game/ModularMedievalNPC/CharacterParts/Blueprints/BP_PartAsset_SK_Leg.BP_PartAsset_SK_Leg_C" :`NewEnumerator4` "/Game/ModularMedievalNPC/CharacterParts/Blueprints/BP_PartAsset_SM_HandItem.BP_PartAsset_SM_HandItem_C" :`NewEnumerator5` "/Game/ModularMedievalNPC/CharacterParts/Blueprints/BP_PartAsset_SM_HandItem.BP_PartAsset_SM_HandItem_C" :!type "/Game/ModularMedievalNPC/CharacterParts/Blueprints/BP_PartAsset Class Reference")))

(fn `GetPartAssetsFromAssetRegistry`
  (params (Class :type "/Game/ModularMedievalNPC/CharacterParts/Blueprints/BP_PartAsset Class Reference") (AddEmptyPartAsset :type Boolean))
  (returns (ReturnValue :type Boolean) (PartAssets :type "Array of /Game/ModularMedievalNPC/CharacterParts/Blueprints/BP_PartAsset Object Reference"))
  (locals (lPartAssets :type "Array of /Game/ModularMedievalNPC/CharacterParts/Blueprints/BP_PartAsset Object Reference"))
  ;[0 0 0] Get Asset by Class from Asset Registry
  (bind _outassetdata (message `AssetRegistry.GetAssetsByClass` (`KismetSystemLibrary.Conv_InterfaceToObject` (`AssetRegistryHelpers.GetAssetRegistry`)) (`KismetStringLibrary.Conv_StringToName` (`KismetSystemLibrary.GetClassDisplayName` Class)) true))
  (for _array_element _outassetdata
    (bind _asbp_part_asset (cast `/Game/ModularMedievalNPC/CharacterParts/Blueprints/BP_PartAsset` (`AssetRegistryHelpers.GetAsset` _array_element)))
    (`KismetArrayLibrary.Array_Add` (`local.lPartAssets`) _asbp_part_asset))
  (`|ExecutionSequence`
    (:`then_0`
      ;[0 0 0] Add an empty Part Asset to the array (e.g. if the slot associated to the part can be empty - Right Hand and Left Hand are examples)
      (if AddEmptyPartAsset
        (`KismetArrayLibrary.Array_Add` (`local.lPartAssets`))))
    (:`then_1`
      (return (> (`KismetArrayLibrary.Array_Length` (`local.lPartAssets`)) 0) (`local.lPartAssets`)))))

(fn `GetPartAssetsFromAssetRegistryByPartTags`
  (params (Class :type "/Game/ModularMedievalNPC/CharacterParts/Blueprints/BP_PartAsset Class Reference") (PartAssetFilter :type "GameplayTagContainer Structure") (ExcludeEmptyPartTags :type Boolean) (AddEmptyPartAsset :type Boolean))
  (returns (ReturnValue :type Boolean) (PartAssets :type "Array of /Game/ModularMedievalNPC/CharacterParts/Blueprints/BP_PartAsset Object Reference"))
  (locals (lPartAssets :type "Array of /Game/ModularMedievalNPC/CharacterParts/Blueprints/BP_PartAsset Object Reference"))
  ;[0 0 0] Get Asset by Class from Asset Registry and by Gameplay Tags
  (bind _outassetdata (message `AssetRegistry.GetAssetsByClass` (`KismetSystemLibrary.Conv_InterfaceToObject` (`AssetRegistryHelpers.GetAssetRegistry`)) (`KismetStringLibrary.Conv_StringToName` (`KismetSystemLibrary.GetClassDisplayName` Class)) true))
  (for _array_element _outassetdata
    (bind _asbp_part_asset (cast `/Game/ModularMedievalNPC/CharacterParts/Blueprints/BP_PartAsset` (`AssetRegistryHelpers.GetAsset` _array_element)))
    (if (<= (`BlueprintGameplayTagLibrary.GetNumGameplayTagsInContainer` PartAssetFilter) 0)
      (`KismetArrayLibrary.Array_Add` (`local.lPartAssets`) _asbp_part_asset :!label _label)
      (else
        (bind _parttags (`/Game/ModularMedievalNPC/CharacterParts/Blueprints/BP_PartAsset.PartTags` _asbp_part_asset))
        (if (<= (`BlueprintGameplayTagLibrary.GetNumGameplayTagsInContainer` _parttags) 0)
          (if (not ExcludeEmptyPartTags)
            (goto _label))
          (elif (`BlueprintGameplayTagLibrary.HasAnyTags` _parttags PartAssetFilter)
            (goto _label))))))
  (`|ExecutionSequence`
    (:`then_0`
      ;[0 0 0] Add an empty Part Asset to the array (e.g. if the slot associated to the part can be empty - Right Hand and Left Hand are examples)
      (if AddEmptyPartAsset
        (`KismetArrayLibrary.Array_Add` (`local.lPartAssets`))))
    (:`then_1`
      (return (> (`KismetArrayLibrary.Array_Length` (`local.lPartAssets`)) 0) (`local.lPartAssets`)))))

(fn `GetRandomPartAssets`
  (returns (Hat :type "/Game/ModularMedievalNPC/CharacterParts/Blueprints/BP_PartAsset_SK_Hat Object Reference") (Hair :type "/Game/ModularMedievalNPC/CharacterParts/Blueprints/BP_PartAsset_SK_Hair Object Reference") (Head :type "/Game/ModularMedievalNPC/CharacterParts/Blueprints/BP_PartAsset_SK_Head Object Reference") (Chest :type "/Game/ModularMedievalNPC/CharacterParts/Blueprints/BP_PartAsset_SK_Chest Object Reference") (Arm :type "/Game/ModularMedievalNPC/CharacterParts/Blueprints/BP_PartAsset_SK_Arm Object Reference") (Leg :type "/Game/ModularMedievalNPC/CharacterParts/Blueprints/BP_PartAsset_SK_Leg Object Reference") (RightHand :type "/Game/ModularMedievalNPC/CharacterParts/Blueprints/BP_PartAsset_SM_HandItem Object Reference") (LeftHand :type "/Game/ModularMedievalNPC/CharacterParts/Blueprints/BP_PartAsset_SM_HandItem Object Reference"))
  (bind ___worldcontext (`local.__WorldContext`))
  (`|ExecutionSequence`
    (:`then_0`
      (bind (_returnvalue _partassets) (`self.GetPartAssetsFromAssetRegistry` "/Game/ModularMedievalNPC/CharacterParts/Blueprints/BP_PartAsset_SK_Hat.BP_PartAsset_SK_Hat_C" false ___worldcontext)) ; Hat
      (if _returnvalue
        (bind _asbp_part_asset_sk_hat (cast `/Game/ModularMedievalNPC/CharacterParts/Blueprints/BP_PartAsset_SK_Hat` (`/Game/ModularMedievalNPC/CharacterParts/Blueprints/BPML_PartAssetHelper.GetRandomArrayElement` _partassets)))
        (bind _get (`/Game/ModularMedievalNPC/CharacterParts/Blueprints/BPML_PartAssetHelper.TempVariable` _asbp_part_asset_sk_hat))))
    (:`then_1`
      (bind (_returnvalue_2 _partassets_2) (`self.GetPartAssetsFromAssetRegistry` "/Game/ModularMedievalNPC/CharacterParts/Blueprints/BP_PartAsset_SK_Hair.BP_PartAsset_SK_Hair_C" false ___worldcontext)) ; Hair
      (if _returnvalue_2
        (bind _asbp_part_asset_sk_hair (cast `/Game/ModularMedievalNPC/CharacterParts/Blueprints/BP_PartAsset_SK_Hair` (`/Game/ModularMedievalNPC/CharacterParts/Blueprints/BPML_PartAssetHelper.GetRandomArrayElement` _partassets_2)))
        (bind _get_2 (`/Game/ModularMedievalNPC/CharacterParts/Blueprints/BPML_PartAssetHelper.TempVariable` _asbp_part_asset_sk_hair))))
    (:`then_2`
      (bind (_returnvalue_3 _partassets_3) (`self.GetPartAssetsFromAssetRegistry` "/Game/ModularMedievalNPC/CharacterParts/Blueprints/BP_PartAsset_SK_Head.BP_PartAsset_SK_Head_C" false ___worldcontext)) ; Head
      (if _returnvalue_3
        (bind _asbp_part_asset_sk_head (cast `/Game/ModularMedievalNPC/CharacterParts/Blueprints/BP_PartAsset_SK_Head` (`/Game/ModularMedievalNPC/CharacterParts/Blueprints/BPML_PartAssetHelper.GetRandomArrayElement` _partassets_3)))
        (bind _get_3 (`/Game/ModularMedievalNPC/CharacterParts/Blueprints/BPML_PartAssetHelper.TempVariable` _asbp_part_asset_sk_head))))
    (:`then_3`
      (bind (_returnvalue_4 _partassets_4) (`self.GetPartAssetsFromAssetRegistry` "/Game/ModularMedievalNPC/CharacterParts/Blueprints/BP_PartAsset_SK_Chest.BP_PartAsset_SK_Chest_C" false ___worldcontext)) ; Chest
      (if _returnvalue_4
        (bind _asbp_part_asset_sk_chest (cast `/Game/ModularMedievalNPC/CharacterParts/Blueprints/BP_PartAsset_SK_Chest` (`/Game/ModularMedievalNPC/CharacterParts/Blueprints/BPML_PartAssetHelper.GetRandomArrayElement` _partassets_4)))
        (bind _get_4 (`/Game/ModularMedievalNPC/CharacterParts/Blueprints/BPML_PartAssetHelper.TempVariable` _asbp_part_asset_sk_chest))))
    (:`then_4`
      (bind (_returnvalue_5 _partassets_5) (`self.GetPartAssetsFromAssetRegistry` "/Game/ModularMedievalNPC/CharacterParts/Blueprints/BP_PartAsset_SK_Arm.BP_PartAsset_SK_Arm_C" false ___worldcontext)) ; Arm
      (if _returnvalue_5
        (bind _asbp_part_asset_sk_arm (cast `/Game/ModularMedievalNPC/CharacterParts/Blueprints/BP_PartAsset_SK_Arm` (`/Game/ModularMedievalNPC/CharacterParts/Blueprints/BPML_PartAssetHelper.GetRandomArrayElement` _partassets_5)))
        (bind _get_5 (`/Game/ModularMedievalNPC/CharacterParts/Blueprints/BPML_PartAssetHelper.TempVariable` _asbp_part_asset_sk_arm))))
    (:`then_5`
      (bind (_returnvalue_6 _partassets_6) (`self.GetPartAssetsFromAssetRegistry` "/Game/ModularMedievalNPC/CharacterParts/Blueprints/BP_PartAsset_SK_Leg.BP_PartAsset_SK_Leg_C" false ___worldcontext)) ; Leg
      (if _returnvalue_6
        (bind _asbp_part_asset_sk_leg (cast `/Game/ModularMedievalNPC/CharacterParts/Blueprints/BP_PartAsset_SK_Leg` (`/Game/ModularMedievalNPC/CharacterParts/Blueprints/BPML_PartAssetHelper.GetRandomArrayElement` _partassets_6)))
        (bind _get_6 (`/Game/ModularMedievalNPC/CharacterParts/Blueprints/BPML_PartAssetHelper.TempVariable` _asbp_part_asset_sk_leg))))
    (:`then_6`
      (bind (_returnvalue_7 _partassets_7) (`self.GetPartAssetsFromAssetRegistry` "/Game/ModularMedievalNPC/CharacterParts/Blueprints/BP_PartAsset_SM_HandItem.BP_PartAsset_SM_HandItem_C" true ___worldcontext)) ; Right Hand
      (if _returnvalue_7
        (bind _asbp_part_asset_sm_hand_item (cast `/Game/ModularMedievalNPC/CharacterParts/Blueprints/BP_PartAsset_SM_HandItem` (`/Game/ModularMedievalNPC/CharacterParts/Blueprints/BPML_PartAssetHelper.GetRandomArrayElement` _partassets_7)))
        (bind _get_7 (`/Game/ModularMedievalNPC/CharacterParts/Blueprints/BPML_PartAssetHelper.TempVariable` _asbp_part_asset_sm_hand_item))))
    (:`then_7`
      (bind (_returnvalue_8 _partassets_8) (`self.GetPartAssetsFromAssetRegistry` "/Game/ModularMedievalNPC/CharacterParts/Blueprints/BP_PartAsset_SM_HandItem.BP_PartAsset_SM_HandItem_C" true ___worldcontext)) ; Left Hand
      (if _returnvalue_8
        (bind _asbp_part_asset_sm_hand_item_2 (cast `/Game/ModularMedievalNPC/CharacterParts/Blueprints/BP_PartAsset_SM_HandItem` (`/Game/ModularMedievalNPC/CharacterParts/Blueprints/BPML_PartAssetHelper.GetRandomArrayElement` _partassets_8)))
        (bind _get_8 (`/Game/ModularMedievalNPC/CharacterParts/Blueprints/BPML_PartAssetHelper.TempVariable` _asbp_part_asset_sm_hand_item_2))))
    (:`then_8`
      (return _get _get_2 _get_3 _get_4 _get_5 _get_6 _get_7 _get_8))))

(fn `GetRandomPartAssetsByPartTags`
  (params (PartAssetFilter :type "GameplayTagContainer Structure") (ExcludeEmptyPartTags :type Boolean))
  (returns (Hat :type "/Game/ModularMedievalNPC/CharacterParts/Blueprints/BP_PartAsset_SK_Hat Object Reference") (Hair :type "/Game/ModularMedievalNPC/CharacterParts/Blueprints/BP_PartAsset_SK_Hair Object Reference") (Head :type "/Game/ModularMedievalNPC/CharacterParts/Blueprints/BP_PartAsset_SK_Head Object Reference") (Chest :type "/Game/ModularMedievalNPC/CharacterParts/Blueprints/BP_PartAsset_SK_Chest Object Reference") (Arm :type "/Game/ModularMedievalNPC/CharacterParts/Blueprints/BP_PartAsset_SK_Arm Object Reference") (Leg :type "/Game/ModularMedievalNPC/CharacterParts/Blueprints/BP_PartAsset_SK_Leg Object Reference") (RightHand :type "/Game/ModularMedievalNPC/CharacterParts/Blueprints/BP_PartAsset_SM_HandItem Object Reference") (LeftHand :type "/Game/ModularMedievalNPC/CharacterParts/Blueprints/BP_PartAsset_SM_HandItem Object Reference"))
  (bind ___worldcontext (`local.__WorldContext`))
  (`|ExecutionSequence`
    (:`then_0`
      (bind (_returnvalue _partassets) (`self.GetPartAssetsFromAssetRegistryByPartTags` "/Game/ModularMedievalNPC/CharacterParts/Blueprints/BP_PartAsset_SK_Hat.BP_PartAsset_SK_Hat_C" PartAssetFilter ExcludeEmptyPartTags false ___worldcontext)) ; Hat
      (if _returnvalue
        (bind _asbp_part_asset_sk_hat (cast `/Game/ModularMedievalNPC/CharacterParts/Blueprints/BP_PartAsset_SK_Hat` (`/Game/ModularMedievalNPC/CharacterParts/Blueprints/BPML_PartAssetHelper.GetRandomArrayElement` _partassets)))
        (bind _get (`/Game/ModularMedievalNPC/CharacterParts/Blueprints/BPML_PartAssetHelper.TempVariable` _asbp_part_asset_sk_hat))))
    (:`then_1`
      (bind (_returnvalue_2 _partassets_2) (`self.GetPartAssetsFromAssetRegistryByPartTags` "/Game/ModularMedievalNPC/CharacterParts/Blueprints/BP_PartAsset_SK_Hair.BP_PartAsset_SK_Hair_C" PartAssetFilter ExcludeEmptyPartTags false ___worldcontext)) ; Hair
      (if _returnvalue_2
        (bind _asbp_part_asset_sk_hair (cast `/Game/ModularMedievalNPC/CharacterParts/Blueprints/BP_PartAsset_SK_Hair` (`/Game/ModularMedievalNPC/CharacterParts/Blueprints/BPML_PartAssetHelper.GetRandomArrayElement` _partassets_2)))
        (bind _get_2 (`/Game/ModularMedievalNPC/CharacterParts/Blueprints/BPML_PartAssetHelper.TempVariable` _asbp_part_asset_sk_hair))))
    (:`then_2`
      (bind (_returnvalue_3 _partassets_3) (`self.GetPartAssetsFromAssetRegistryByPartTags` "/Game/ModularMedievalNPC/CharacterParts/Blueprints/BP_PartAsset_SK_Head.BP_PartAsset_SK_Head_C" PartAssetFilter ExcludeEmptyPartTags false ___worldcontext)) ; Head
      (if _returnvalue_3
        (bind _asbp_part_asset_sk_head (cast `/Game/ModularMedievalNPC/CharacterParts/Blueprints/BP_PartAsset_SK_Head` (`/Game/ModularMedievalNPC/CharacterParts/Blueprints/BPML_PartAssetHelper.GetRandomArrayElement` _partassets_3)))
        (bind _get_3 (`/Game/ModularMedievalNPC/CharacterParts/Blueprints/BPML_PartAssetHelper.TempVariable` _asbp_part_asset_sk_head))))
    (:`then_3`
      (bind (_returnvalue_4 _partassets_4) (`self.GetPartAssetsFromAssetRegistryByPartTags` "/Game/ModularMedievalNPC/CharacterParts/Blueprints/BP_PartAsset_SK_Chest.BP_PartAsset_SK_Chest_C" PartAssetFilter ExcludeEmptyPartTags false ___worldcontext)) ; Chest
      (if _returnvalue_4
        (bind _asbp_part_asset_sk_chest (cast `/Game/ModularMedievalNPC/CharacterParts/Blueprints/BP_PartAsset_SK_Chest` (`/Game/ModularMedievalNPC/CharacterParts/Blueprints/BPML_PartAssetHelper.GetRandomArrayElement` _partassets_4)))
        (bind _get_4 (`/Game/ModularMedievalNPC/CharacterParts/Blueprints/BPML_PartAssetHelper.TempVariable` _asbp_part_asset_sk_chest))))
    (:`then_4`
      (bind (_returnvalue_5 _partassets_5) (`self.GetPartAssetsFromAssetRegistryByPartTags` "/Game/ModularMedievalNPC/CharacterParts/Blueprints/BP_PartAsset_SK_Arm.BP_PartAsset_SK_Arm_C" PartAssetFilter ExcludeEmptyPartTags false ___worldcontext)) ; Arm
      (if _returnvalue_5
        (bind _asbp_part_asset_sk_arm (cast `/Game/ModularMedievalNPC/CharacterParts/Blueprints/BP_PartAsset_SK_Arm` (`/Game/ModularMedievalNPC/CharacterParts/Blueprints/BPML_PartAssetHelper.GetRandomArrayElement` _partassets_5)))
        (bind _get_5 (`/Game/ModularMedievalNPC/CharacterParts/Blueprints/BPML_PartAssetHelper.TempVariable` _asbp_part_asset_sk_arm))))
    (:`then_5`
      (bind (_returnvalue_6 _partassets_6) (`self.GetPartAssetsFromAssetRegistryByPartTags` "/Game/ModularMedievalNPC/CharacterParts/Blueprints/BP_PartAsset_SK_Leg.BP_PartAsset_SK_Leg_C" PartAssetFilter ExcludeEmptyPartTags false ___worldcontext)) ; Leg
      (if _returnvalue_6
        (bind _asbp_part_asset_sk_leg (cast `/Game/ModularMedievalNPC/CharacterParts/Blueprints/BP_PartAsset_SK_Leg` (`/Game/ModularMedievalNPC/CharacterParts/Blueprints/BPML_PartAssetHelper.GetRandomArrayElement` _partassets_6)))
        (bind _get_6 (`/Game/ModularMedievalNPC/CharacterParts/Blueprints/BPML_PartAssetHelper.TempVariable` _asbp_part_asset_sk_leg))))
    (:`then_6`
      (bind (_returnvalue_7 _partassets_7) (`self.GetPartAssetsFromAssetRegistryByPartTags` "/Game/ModularMedievalNPC/CharacterParts/Blueprints/BP_PartAsset_SM_HandItem.BP_PartAsset_SM_HandItem_C" PartAssetFilter ExcludeEmptyPartTags true)) ; Right Hand
      (if _returnvalue_7
        (bind _asbp_part_asset_sm_hand_item (cast `/Game/ModularMedievalNPC/CharacterParts/Blueprints/BP_PartAsset_SM_HandItem` (`/Game/ModularMedievalNPC/CharacterParts/Blueprints/BPML_PartAssetHelper.GetRandomArrayElement` _partassets_7)))
        (bind _get_7 (`/Game/ModularMedievalNPC/CharacterParts/Blueprints/BPML_PartAssetHelper.TempVariable` _asbp_part_asset_sm_hand_item))))
    (:`then_7`
      (bind (_returnvalue_8 _partassets_8) (`self.GetPartAssetsFromAssetRegistryByPartTags` "/Game/ModularMedievalNPC/CharacterParts/Blueprints/BP_PartAsset_SM_HandItem.BP_PartAsset_SM_HandItem_C" PartAssetFilter ExcludeEmptyPartTags true)) ; Left Hand
      (if _returnvalue_8
        (bind _asbp_part_asset_sm_hand_item_2 (cast `/Game/ModularMedievalNPC/CharacterParts/Blueprints/BP_PartAsset_SM_HandItem` (`/Game/ModularMedievalNPC/CharacterParts/Blueprints/BPML_PartAssetHelper.GetRandomArrayElement` _partassets_8)))
        (bind _get_8 (`/Game/ModularMedievalNPC/CharacterParts/Blueprints/BPML_PartAssetHelper.TempVariable` _asbp_part_asset_sm_hand_item_2))))
    (:`then_8`
      (return _get _get_2 _get_3 _get_4 _get_5 _get_6 _get_7 _get_8))))

(fn `SortByDisplayNameFromA_toZ`
  (params (PartAssets :type "Array of /Game/ModularMedievalNPC/CharacterParts/Blueprints/BP_PartAsset Object Reference"))
  (returns (ReturnValue :type "Array of /Game/ModularMedievalNPC/CharacterParts/Blueprints/BP_PartAsset Object Reference"))
  (locals (lPartAssetsSorted :type "Array of /Game/ModularMedievalNPC/CharacterParts/Blueprints/BP_PartAsset Object Reference") (lPartAssetDisplayNamesUnsorted :type "Array of String") (lPartAssetDisplayNamesSorted :type "Array of String") (InsertionIndex :type Integer :default 0) (lPartAssetsUnsorted :type "Array of /Game/ModularMedievalNPC/CharacterParts/Blueprints/BP_PartAsset Object Reference"))
  (set `local.lPartAssetsUnsorted` PartAssets)
  (`|ExecutionSequence`
    (:`then_0`
      ;[0 0 0] Save Display Names of the unsorted Part Assets
      (for _array_element (`local.lPartAssetsUnsorted`)
        (`KismetArrayLibrary.Array_Add` (`local.lPartAssetDisplayNamesUnsorted`) (`KismetTextLibrary.Conv_TextToString` (`/Game/ModularMedievalNPC/CharacterParts/Blueprints/BP_PartAsset.DisplayName` _array_element)))))
    (:`then_1`
      ;[0 0 0] Foreach DisplayNames element:
      ; Sort in alphabetical order into a DisplayNamesSorted array.
      (for (_array_element_2 _array_index) (`local.lPartAssetDisplayNamesUnsorted`)
        ;;[1 1 1] Foreach existing DisplayNamesSorted element:
        ;; Check if the current DisplayNamesSorted element's characters' ASCII values are >, == or < than the current DisplayNames element's ASCII value.
        (for (_array_element_3 _array_index_2) (`local.lPartAssetDisplayNamesSorted`) :!label _label
          (set `local.InsertionIndex` _array_index_2)
          ;;;[1 1 1] Check each single character's ASCII value
          (for _index (range (+ (`KismetStringLibrary.Len` _array_element_2) 1))
            (`/Engine/EditorBlueprintResources/StandardMacros.CompareInt` (`KismetStringLibrary.GetCharacterAsNumber` _array_element_3 _index) (`KismetStringLibrary.GetCharacterAsNumber` _array_element_2 _index) ; >   ASCII value of Sorted Element is larger than Unsorted Element:\n       Break the character comparison and break checking the next Sorted Element,\n       to insert the current Unsorted Element before the next Sorted Element.\n\n==   ASCII values are equal, go to next character\n\n  <   ASCII value of Sorted Element is smaller than Unsorted Element:\n        Break the character comparison and go to next Sorted Element, but\n        at first increase InsertionIndex, in case this was the last Sorted Element.
              (:`>`
                (`|ExecutionSequence`
                  (:`then_0`
                    (break))
                  (:`then_1`
                    (goto _label :!via `Break`))))
              (:`<`
                (`/Engine/EditorBlueprintResources/StandardMacros.IncrementInt` (`local.InsertionIndex`)
                  (:`  `
                    (break)))))))
        ;;;[1 1 1] Add to DisplayNamesSorted for the next DisplayNames element.
        (`KismetArrayLibrary.Array_Insert` (`local.lPartAssetDisplayNamesSorted`) _array_element_2 (`local.InsertionIndex`))
        ;;;[1 1 1] Use the same Insertion Index to sort the Part Asset associated to the Display Name.
        (`KismetArrayLibrary.Array_Insert` (`local.lPartAssetsSorted`) (`|GetArrayItem` (`local.lPartAssetsUnsorted`) _array_index) (`local.InsertionIndex`))))
    (:`then_2`
      (return (`local.lPartAssetsSorted`)))))