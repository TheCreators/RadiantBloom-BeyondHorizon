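; Character component that lets the player plant hotbar seeds on growing plots and water, fertilize, damage or interact with plants.
; A camera-forward sphere trace finds targets, which actions reach through BPI_Farming or ApplyDamage.
; On BeginPlay, the server respawns non-hand-placed plants from FarmSave and relinks their pluckable yields by GUID.
; Demo animations and held meshes replicate through RepNotifies, with an incrementing counter so repeated animations still fire.
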(event `self.ReceiveBeginPlay`
  (`|ExecutionSequence`
    (:`then_0`
      ;[0 1 0.6484] Store character and camera reference
      (bind _ascharacter (cast `Character` (`self.GetOwner`)))
      (bind _output_get (set `self.Owning character referemce` _ascharacter))
      (set `self.Camera Reference` (`Actor.GetComponentByClass` _output_get "/Script/Engine.CameraComponent")))
    (:`then_1`
      ;[0 1 0.1094] Load farming
      (`self.Load Farming`))))

(event `Event: Spawn Seed`
  (params (SpawnTransform :type "Transform Structure") (Plant :type "DataTableRowHandle Structure (by ref)"))
  (bind (_datatable _rowname) (break `DataTableRowHandle` Plant))
  ;[0.2188 0 1] Spawn Seed
  (bind _returnvalue (`|GetDataTableRow` _datatable _rowname)
    (:`then`
      ;;[0.2422 1 0] Spawn the specific actor(plant type)
      (bind _asbp_farming_master (castclass `/Game/FarmingSystem/Blueprints/Masters/BP_Farming_Master` (`.Actortospawn_13_83D256BD44F7DFEC0B33508A1590FF91` (break `/Game/FarmingSystem/Datamodel/Substructs/Struct_PlantAttributes_Generic` (`.Generic_82_923D547C4DB182B1CF7DC4917D8485DA` (break `/Game/FarmingSystem/Datamodel/Struct_Plant` _returnvalue))))))
      (`|SpawnActorFromClass` :`Class` _asbp_farming_master :`SpawnTransform` SpawnTransform :`CollisionHandlingOverride` "AlwaysSpawn" :`TransformScaleMethod` "SelectDefaultAtRuntime" :`Plant` Plant :`Instigator` null))))

(event `Spawn Seed on trace location`
  ;[0.2188 0 1] Spawn Seed
  (bind (_hitactor _hitcomponent _hit _outhit) (`self.Trace` "TraceTypeQuery1"))
  (if _hit
    ;;[0.05469 0 1] Only place when looked at actor is growning plot
    (if (`Actor.ActorHasTag` _hitactor "Growing_Plot")
      (bind (_farmable _is_farmable_found _inventory_index) (`self.Get Farmable`))
      (if _is_farmable_found
        (`/Game/Inventory/BPC_InventorySystem.Remove from Inventory` (`/Game/ThirdPerson/Blueprints/BP_ThirdPersonCharacter.BPC_InventorySystem` (cast `/Game/ThirdPerson/Blueprints/BP_ThirdPersonCharacter` (`GameplayStatics.GetPlayerCharacter` 0) :!pure true)) _inventory_index false true)
        (`self.Event: Spawn Seed` (`KismetMathLibrary.MakeTransform` (`.ImpactPoint` (`GameplayStatics.BreakHitResult` _outhit))) _farmable)))))

(event `Play Animation`
  (params (`Animation to play` :type "AnimSequenceBase Object Reference"))
  ;[0 0.6484 1] For show, an animation and mesh showing. In your own system you will want to equip items, and show your animation integrated in your own framework
  ;;[1 0 0.6562] Play a dynamic animation montage.
  ;; Network peformance wise you do not want to use a multicast but want to replicate the action from server to client.
  ;; Rep Notifies are only triggered if the variables are changed. That is why we use a workarround to play each animation via notify of the animation amounts played (always an unique number and therefore notified)
  ;; In Unreal the notofication runs as well on the server as on the clients (in replication radius)
  (set `self.Animation To Play` `Animation to play`)
  (set `self.Amount of animations played` (+ (`self.Amount of animations played`) 1)))

(event `Spawn_Mesh`
  (params (Mesh :type "StaticMesh Object Reference"))
  (bind _current__equiped_mesh (`self.Current  Equiped Mesh`))
  ;[0 0.6484 1] For show, an animation and mesh showing. In your own system you will want to equip items, and show your animation integrated in your own framework
  ;;[0.4531 0 1] Show a mesh for 2 second.
  (`/Engine/EditorBlueprintResources/StandardMacros.IsValid` _current__equiped_mesh
    (:`Is Valid`
      (if (!= _current__equiped_mesh Mesh)
        (set `self.Current  Equiped Mesh` null)
        (set `self.Current  Equiped Mesh` Mesh :!label _label)
        (`KismetSystemLibrary.Delay` 5.0)
        (set `self.Current  Equiped Mesh` null)))
    (:`Is Not Valid`
      (goto _label))))

(event `Event: Spawn Plants from save`
  ;[0 1 0.5078] spawn from save if server and we only want to do it once, so only character 0 excecutes this function
  (`self.Spawn_Plants_From_Save`))

(event `Load Farming`
  ;[0 1 0.5078] spawn from save if server and we only want to do it once, so only character 0 excecutes this function
  (if (and (`KismetSystemLibrary.IsServer`) (`Pawn.IsControlled` (`self.Owning character referemce`)))
    (`/Engine/EditorBlueprintResources/StandardMacros.IsValid` (`GameplayStatics.GetPlayerCharacter` 0) :!label _label_2
      (:`Is Valid`
        (`self.Event: Spawn Plants from save`)))
    (elif (`KismetSystemLibrary.IsDedicatedServer`)
      (goto _label_2))))

(event `Event: Try add Fertilizer`
  ;[0.07888 1 0] All interactions with the plants. All logic is done on the server
  (bind _hitactor (`self.Trace` "TraceTypeQuery3"))
  (if (`KismetSystemLibrary.DoesImplementInterface` _hitactor "/Game/FarmingSystem/Blueprints/BPI_Farming.BPI_Farming_C")
    (bind _asplayer_controller (cast `PlayerController` (`Pawn.GetController` (`self.Owning character referemce`))))
    (message `/Game/FarmingSystem/Blueprints/BPI_Farming.Try_Add_Fertilizer` _hitactor 25.0 _asplayer_controller)
    (`self.Play Animation` "/Game/ResourcePack/Animations/State_Animations/Anim_grab.Anim_grab")
    (`self.Spawn_Mesh` "/Game/ResourcePack/Raw_Resources/Open_Sack/Meshes/SM_Open_Sack_Fertilizer_Small.SM_Open_Sack_Fertilizer_Small")))

(event `Event: Try add Water`
  ;[0.07888 1 0] All interactions with the plants. All logic is done on the server
  (bind _hitactor (`self.Trace` "TraceTypeQuery3"))
  (if (`KismetSystemLibrary.DoesImplementInterface` _hitactor "/Game/FarmingSystem/Blueprints/BPI_Farming.BPI_Farming_C")
    (bind _asplayer_controller (cast `PlayerController` (`Pawn.GetController` (`self.Owning character referemce`))))
    (message `/Game/FarmingSystem/Blueprints/BPI_Farming.Try_Add_Water` _hitactor 25.0 _asplayer_controller)
    (`self.Play Animation` "/Game/ResourcePack/Animations/State_Animations/Anim_grab.Anim_grab")
    (`self.Spawn_Mesh` "/Game/ResourcePack/Tools/Watering_Can/SM_Watering_Can.SM_Watering_Can")))

(event `Event: Try Apply Damage`
  ;[0.07888 1 0] All interactions with the plants. All logic is done on the server
  (bind _hitactor (`self.Trace` "TraceTypeQuery3"))
  (if (`KismetSystemLibrary.DoesImplementInterface` _hitactor "/Game/FarmingSystem/Blueprints/BPI_Farming.BPI_Farming_C")
    (bind _asplayer_controller (cast `PlayerController` (`Pawn.GetController` (`self.Owning character referemce`))))
    (`GameplayStatics.ApplyDamage` _hitactor 25.0 null _asplayer_controller)
    (`self.Play Animation` "/Game/ResourcePack/Animations/Melee/Anim_swing_sword_sidewards.Anim_swing_sword_sidewards")
    (`self.Spawn_Mesh` "/Game/ResourcePack/Weapons/Swords/SM_Sword_Steel.SM_Sword_Steel")))

(event `Event: Interact`
  ;[0.07888 1 0] All interactions with the plants. All logic is done on the server
  (bind _hitactor (`self.Trace` "TraceTypeQuery3"))
  (if (`KismetSystemLibrary.DoesImplementInterface` _hitactor "/Game/FarmingSystem/Blueprints/BPI_Farming.BPI_Farming_C")
    (bind _asplayer_controller (cast `PlayerController` (`Pawn.GetController` (`self.Owning character referemce`))))
    (message `/Game/FarmingSystem/Blueprints/BPI_Farming.Interact` _hitactor _asplayer_controller)
    (`self.Play Animation` "/Game/ResourcePack/Animations/State_Animations/Anim_grab.Anim_grab")
    (`self.Spawn_Mesh` "/Game/ResourcePack/Props/Basket/Mesh/SM_Basket_Small.SM_Basket_Small")))

(event `Enable Movement`
  (`CharacterMovementComponent.SetMovementMode` (`Character.CharacterMovement` (cast `/Game/ThirdPerson/Blueprints/BP_ThirdPersonCharacter` (`GameplayStatics.GetPlayerCharacter` 0) :!pure true)) "MOVE_Walking" 0))

(fn `Get Farmable`
  (returns (Farmable :type "DataTableRowHandle Structure") (`Is Farmable Found` :type Boolean) (`Inventory Index` :type Integer))
  (locals (`Local Active Item Name` :type Name))
  (bind _asbp_third_person_character (cast `/Game/ThirdPerson/Blueprints/BP_ThirdPersonCharacter` (`GameplayStatics.GetPlayerCharacter` 0) :!pure true))
  (bind _inventory_index (`/Game/Inventory/UI/WB_Hotbar.Get Active Slot Inventory Index` (`/Game/UI/WB_HUD.Hotbar` (`/Game/ThirdPerson/Blueprints/BP_ThirdPersonCharacter.HUD Widget` _asbp_third_person_character))))
  (bind (_output_itemid _output_quantity) (break `/Game/Inventory/S_InventorySlot` (`|GetArrayItem` (`/Game/Inventory/BPC_InventorySystem.Content` (`/Game/ThirdPerson/Blueprints/BP_ThirdPersonCharacter.BPC_InventorySystem` _asbp_third_person_character)) _inventory_index)))
  (if (<= _output_quantity 0)
    (return (struct) false 0)
    (else
      (set `local.Local Active Item Name` _output_itemid)
      (bind _outrownames (`DataTableFunctionLibrary.GetDataTableRowNames` "/Game/FarmingSystem/Datamodel/DT_Farmables.DT_Farmables"))
      (for _array_element _outrownames
        (bind _returnvalue (`|GetDataTableRow` "/Game/FarmingSystem/Datamodel/DT_Farmables.DT_Farmables" _array_element)
          (:`then`
            (if (== (`.RowName` (break `DataTableRowHandle` (`.Item_94_E891C5AA41E529C1172A28ABEC46F103` (break `/Game/FarmingSystem/Datamodel/Struct_Plant` _returnvalue)))) (`local.Local Active Item Name`))
              (return (make `DataTableRowHandle` "/Game/FarmingSystem/Datamodel/DT_Farmables.DT_Farmables" _array_element) true _inventory_index)))))
      (return (struct) false 0))))

(fn `OnRep_Amount of animations played`
  (bind _animation_to_play (`self.Animation To Play`))
  (`AnimInstance.PlaySlotAnimationAsDynamicMontage` (`SkeletalMeshComponent.GetAnimInstance` (`Character.Mesh` (`self.Owning character referemce`))) _animation_to_play "DefaultSlot" 0.25 0.25 1.0 1 -1.0 0.0)
  (`CharacterMovementComponent.SetMovementMode` (`Character.CharacterMovement` (cast `/Game/ThirdPerson/Blueprints/BP_ThirdPersonCharacter` (`GameplayStatics.GetPlayerCharacter` 0) :!pure true)) "MOVE_None" 0)
  (`KismetSystemLibrary.K2_SetTimerDelegate` (`|CreateDelegate` :!event `Enable Movement`) (`AnimSequenceBase.SequenceLength` _animation_to_play)))

(fn `OnRep_Current  Equiped Mesh`
  (locals (`Local Socket` :type Name))
  (bind _current_attached_actor (`self.Current_Attached_Actor`))
  (bind _current_attached_actor_2 (`self.Current_Attached_Actor`))
  (bind _current__equiped_mesh (`self.Current  Equiped Mesh`))
  (`/Engine/EditorBlueprintResources/StandardMacros.IsValid` (`self.Current  Equiped Mesh`)
    (:`Is Valid`
      (`/Engine/EditorBlueprintResources/StandardMacros.IsValid` _current_attached_actor
        (:`Is Valid`
          (`Actor.K2_DestroyActor` _current_attached_actor))
        (:`Is Not Valid`
          _))
      (bind _returnvalue (`|SpawnActorFromClass` "/Game/FarmingSystem/Character/Blueprints/BP_Dummy_Equipment.BP_Dummy_Equipment_C" (`KismetMathLibrary.MakeTransform` (0.0 0.0 0.0)) "Undefined" "OverrideRootScale" null (`self.Current  Equiped Mesh`) null))
      (if (== _current__equiped_mesh "/Game/ResourcePack/Raw_Resources/Open_Sack/Meshes/SM_Open_Sack_Fertilizer_Small.SM_Open_Sack_Fertilizer_Small")
        (set `local.Local Socket` "Hand_R_Sack")
        (`Actor.K2_AttachToComponent` _returnvalue (`/Game/ThirdPerson/Blueprints/BP_ThirdPersonCharacter.FantasyGirl` (cast `/Game/ThirdPerson/Blueprints/BP_ThirdPersonCharacter` (`GameplayStatics.GetPlayerCharacter` 0) :!pure true)) (`local.Local Socket`) "SnapToTarget" "SnapToTarget" "SnapToTarget" true :!label _label)
        (set `self.Current_Attached_Actor` _returnvalue)
        (elif (== _current__equiped_mesh "/Game/ResourcePack/Props/Basket/Mesh/SM_Basket_Small.SM_Basket_Small")
          (set `local.Local Socket` "Hand_R_Basket")
          (goto _label)
          (elif (== _current__equiped_mesh "/Game/ResourcePack/Tools/Watering_Can/SM_Watering_Can.SM_Watering_Can")
            (set `local.Local Socket` "Hand_R_WateringCan")
            (goto _label)))))
    (:`Is Not Valid`
      (`/Engine/EditorBlueprintResources/StandardMacros.IsValid` _current_attached_actor_2
        (:`Is Valid`
          (`Actor.K2_DestroyActor` _current_attached_actor_2))))))

(fn `Spawn_Plants_From_Save`
  (locals (`Local Save` :type "/Game/FarmingSystem/Save/BP_Save_Plants Object Reference") (`Local  Spawned Plants` :type "Array of /Game/FarmingSystem/Blueprints/Masters/BP_Farming_Master Object Reference") (Local_GUID_To_Actor :type "Map of String to Actor Object Reference"))
  (bind _returnvalue (`GameplayStatics.DoesSaveGameExist` "FarmSave"))
  (if _returnvalue
    (bind _returnvalue_2 (`GameplayStatics.LoadGameFromSlot` "FarmSave"))
    (bind _asbp_save_plants (cast `/Game/FarmingSystem/Save/BP_Save_Plants` _returnvalue_2))
    (set `local.Local Save` _asbp_save_plants)
    (for _array_element (`/Game/FarmingSystem/Save/BP_Save_Plants.Plants` _asbp_save_plants)
      (bind (_guid_farmable _plantdatatablerow _transform _currentdurabilityfarmable _is_regrowing _can_be_harvested _current_growth_stage _current_growth_time _currentamountoffertilizer _currentamountofwater _is_destructed _current_decay_time _is_decayed _is_decaying _is_sick _fertilizerconsumed _linkedpluckableyield _current_growth_percentage _actor _ismanuallyplacedinworld) (break `/Game/FarmingSystem/Save/Struct_Saved_Plants` _array_element))
      (if (not _ismanuallyplacedinworld)
        (bind _asbp_farming_master (castclass `/Game/FarmingSystem/Blueprints/Masters/BP_Farming_Master` _actor))
        (bind _returnvalue_3 (`|SpawnActorFromClass` _asbp_farming_master _transform "AlwaysSpawn" "SelectDefaultAtRuntime" null _current_growth_time _current_growth_stage _current_growth_percentage _plantdatatablerow _can_be_harvested _is_regrowing _is_destructed _currentdurabilityfarmable _guid_farmable _current_decay_time _currentamountoffertilizer _currentamountofwater _is_decayed _is_sick _is_decaying _fertilizerconsumed _linkedpluckableyield true _ismanuallyplacedinworld false true null))
        (`BlueprintMapLibrary.Map_Add` (`local.Local_GUID_To_Actor`) _guid_farmable _returnvalue_3)
        (`KismetArrayLibrary.Array_Add` (`local.Local  Spawned Plants`) _returnvalue_3)))
    (for _array_element_2 (`local.Local  Spawned Plants`)
      (for _array_element_3 (`/Game/FarmingSystem/Blueprints/Masters/BP_Farming_Master.Linked_Pluckable_Yield_GUIDS` _array_element_2)
        (bind (_value _returnvalue_4) (`BlueprintMapLibrary.Map_Find` (`local.Local_GUID_To_Actor`) _array_element_3))
        (if _returnvalue_4
          (`KismetArrayLibrary.Array_Add` (`/Game/FarmingSystem/Blueprints/Masters/BP_Farming_Master.Linked_Pluckable_Yield` _array_element_2) _value))))))

(fn `Trace`
  (params (TraceChannel :type "ETraceTypeQuery Enum" :default "TraceTypeQuery1"))
  (returns (HitActor :type "Actor Object Reference") (HitComponent :type "PrimitiveComponent Object Reference") (Hit :type Boolean) (OutHit :type "HitResult Structure"))
  (bind _camera_reference (`self.Camera Reference`))
  (bind _returnvalue (`SceneComponent.GetForwardVector` _camera_reference))
  (bind _returnvalue_2 (+ (`SceneComponent.K2_GetComponentLocation` _camera_reference) (0.0 0.0 80.0)))
  ;[1 1 1] Trace from camera. Used for multiple purposes throughout the sytem
  (bind (_outhit _returnvalue_3) (`KismetSystemLibrary.SphereTraceSingle` (+ _returnvalue_2 (* _returnvalue 250.0)) (+ _returnvalue_2 (* _returnvalue 1000.0)) 40.0 TraceChannel))
  (bind (_bblockinghit _binitialoverlap _time _distance _location _impactpoint _normal _impactnormal _physmat _hitactor _hitcomponent) (`GameplayStatics.BreakHitResult` _outhit))
  (return _hitactor _hitcomponent _returnvalue_3 _outhit))