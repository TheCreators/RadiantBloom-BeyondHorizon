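; Interactable farming plot where the player plants the seed held in the active hotbar slot.
; The item is matched against DT_Farmables to drive the "Plant {Seeds}" prompt; interacting consumes one and spawns its BP_Farming_Master actor.
; While planted, the plot's box ignores a custom collision channel, restored when the spawned plant is destroyed.
; A sphere trace one tick after BeginPlay detects an existing plant to set the initial state.
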(event `self.ReceiveBeginPlay`
  ;[0.7813 0 1] Get Character BP
  (bind _asbp_third_person_character (cast `/Game/ThirdPerson/Blueprints/BP_ThirdPersonCharacter` (`GameplayStatics.GetPlayerCharacter` 0)))
  (set `self.Character BP` _asbp_third_person_character)
  ;[0 1 0.8125] Check for plant
  (`KismetSystemLibrary.DelayUntilNextTick`)
  (if (`self.Find Plant`)
    (`self.Set Plant Exist`)
    (else
      (`self.Set Plant Not Exist`))))

(event `/Game/InteractionSystem/BPI_Interact.Interact With`
  (params (`Player Character` :type "/Game/ThirdPerson/Blueprints/BP_ThirdPersonCharacter Object Reference"))
  ;[0 1 0.2031] Interaction
  (`self.Try Plant`))

(event `On Plant Destory`
  (params (DestroyedActor :type "Actor Object Reference"))
  ;[0 1 0.2031] Interaction
  (`self.Set Plant Not Exist`))

(fn `Can Interact With`
  (returns (`Can Interact` :type Boolean))
  (return (and (`.Is Farmable Found` (`self.Get Farmable`)) (not (`self.Has Plant`)))))

(fn `Find Plant`
  (returns (Found :type Boolean))
  (bind _returnvalue (`SceneComponent.K2_GetComponentLocation` (`self.Plant Location`)))
  (bind (_outhit _returnvalue_2) (`KismetSystemLibrary.SphereTraceSingle` _returnvalue _returnvalue 30.0 "TraceTypeQuery3"))
  (if _returnvalue_2
    (cast `/Game/FarmingSystem/Blueprints/Masters/BP_Farming_Master` (`.HitActor` (`GameplayStatics.BreakHitResult` _outhit))
      (:`then`
        (return true))
      (:`CastFailed`
        _)))
  (return false))

(fn `Get Farmable`
  (returns (Farmable :type "DataTableRowHandle Structure") (`Is Farmable Found` :type Boolean) (`Inventory Index` :type Integer))
  (locals (`Local Active Item Name` :type Name))
  (bind _character_bp (`self.Character BP`))
  (bind _inventory_index (`/Game/Inventory/UI/WB_Hotbar.Get Active Slot Inventory Index` (`/Game/UI/WB_HUD.Hotbar` (`/Game/ThirdPerson/Blueprints/BP_ThirdPersonCharacter.HUD Widget` _character_bp))))
  (bind (_output_itemid _output_quantity) (break `/Game/Inventory/S_InventorySlot` (`|GetArrayItem` (`/Game/Inventory/BPC_InventorySystem.Content` (`/Game/ThirdPerson/Blueprints/BP_ThirdPersonCharacter.BPC_InventorySystem` _character_bp)) _inventory_index)))
  (if (<= _output_quantity 0)
    (return (struct) false 0)
    (else
      (set `local.Local Active Item Name` _output_itemid)
      (bind _outrownames (`DataTableFunctionLibrary.GetDataTableRowNames` "/Game/FarmingSystem/Datamodel/DT_Farmables.DT_Farmables"))
      (for _array_element _outrownames
        (bind _returnvalue (`|GetDataTableRow` "/Game/FarmingSystem/Datamodel/DT_Farmables.DT_Farmables" _array_element)
          (:`then`
            (if (== (`.RowName` (break `DataTableRowHandle` (`.Item_94_E891C5AA41E529C1172A28ABEC46F103` (break `/Game/FarmingSystem/Datamodel/Struct_Plant` _returnvalue)))) (`local.Local Active Item Name`))
              (return (make `DataTableRowHandle` "/Game/FarmingSystem/Datamodel/DT_Farmables.DT_Farmables" _array_element) true _inventory_index)))))
      (return (struct) false 0))))

(fn `Get Meshes To Outline`
  (returns (Meshes :type "Set of MeshComponent Object Reference"))
  (return (`|MakeSet` (`self.Mesh`) :!type "MeshComponent Object Reference")))

(fn `Look At`
  (returns (Message :type Text))
  (bind (_farmable _is_farmable_found) (`self.Get Farmable`))
  (bind (_datatable _rowname) (break `DataTableRowHandle` _farmable))
  (if (and _is_farmable_found (not (`self.Has Plant`)))
    (bind _returnvalue (`|GetDataTableRow` _datatable _rowname)
      (:`then`
        (return (`|FormatText` "Plant {Seeds}" (`.Name_2_3DE19FA64157CA393A5581947AAA309E` (break `/Game/FarmingSystem/Datamodel/Substructs/Struct_PlantAttributes_Generic` (`.Generic_82_923D547C4DB182B1CF7DC4917D8485DA` (break `/Game/FarmingSystem/Datamodel/Struct_Plant` _returnvalue))))))))))

(fn `Set Plant Exist`
  (set `self.Has Plant` true)
  (`PrimitiveComponent.SetCollisionResponseToChannel` (`self.Box Collider`) "ECC_GameTraceChannel1" "ECR_Ignore"))

(fn `Set Plant Not Exist`
  (set `self.Has Plant` false)
  (`PrimitiveComponent.SetCollisionResponseToChannel` (`self.Box Collider`) "ECC_GameTraceChannel1" "ECR_Block"))

(fn `Try Plant`
  (locals (`Local Farmable` :type "DataTableRowHandle Structure"))
  (bind (_farmable _is_farmable_found _inventory_index) (`self.Get Farmable`))
  (bind (_local_farmable_datatable _local_farmable_rowname) (break `DataTableRowHandle` (`local.Local Farmable`)))
  (if _is_farmable_found
    (set `local.Local Farmable` _farmable)
    (`/Game/Inventory/BPC_InventorySystem.Remove from Inventory` (`/Game/ThirdPerson/Blueprints/BP_ThirdPersonCharacter.BPC_InventorySystem` (`self.Character BP`)) _inventory_index false true)
    (bind _returnvalue (`|GetDataTableRow` _local_farmable_datatable _local_farmable_rowname)
      (:`then`
        (bind _asbp_farming_master (castclass `/Game/FarmingSystem/Blueprints/Masters/BP_Farming_Master` (`.Actortospawn_13_83D256BD44F7DFEC0B33508A1590FF91` (break `/Game/FarmingSystem/Datamodel/Substructs/Struct_PlantAttributes_Generic` (`.Generic_82_923D547C4DB182B1CF7DC4917D8485DA` (break `/Game/FarmingSystem/Datamodel/Struct_Plant` _returnvalue))))))
        (bind _returnvalue_2 (`|SpawnActorFromClass` :`Class` _asbp_farming_master :`SpawnTransform` (`KismetMathLibrary.MakeTransform` (`SceneComponent.K2_GetComponentLocation` (`self.Plant Location`))) :`CollisionHandlingOverride` "AlwaysSpawn" :`TransformScaleMethod` "SelectDefaultAtRuntime" :`Plant` (`local.Local Farmable`) :`Instigator` null))
        (`self.Set Plant Exist`)
        (add `self.OnDestroyed` _returnvalue_2 (`|CreateDelegate` :!event `On Plant Destory`))))))

(fn `UserConstructionScript`)