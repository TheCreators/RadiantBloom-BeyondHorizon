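; BP_Sprinkler is an interactable farming sprinkler that registers itself as a water source with farming masters inside its sphere radius.
; Interacting toggles it on the server, requiring HasWater to switch on, while OnRep_Is_On drives audio and particles.
; It adds or removes itself on overlapping farmables at BeginPlay, toggle and destruction, and re-registers on new overlaps while on.
; A GUID is generated at BeginPlay if empty.
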(event `self.ReceiveBeginPlay`
  (bind _is_on (`self.Is_On`))
  (`/Engine/EditorBlueprintResources/ActorMacros.Switch Has Authority`
    (:`Authority`
      ;[1 1 1] At initialize, store GUID and set the sprinkler on or off and also propegate this to the overlapping farming masters
      (`self.Get GUID`)
      (set `self.Is_On` _is_on)
      (if _is_on
        (`self.Set is watered by sprinkler in sprinkler radius` true)
        (else
          (`self.Set is watered by sprinkler in sprinkler radius` false))))))

(event `self.Sphere.OnComponentBeginOverlap`
  (params (OverlappedComponent :type "PrimitiveComponent Object Reference") (OtherActor :type "Actor Object Reference") (OtherComp :type "PrimitiveComponent Object Reference") (OtherBodyIndex :type Integer) (bFromSweep :type Boolean) (SweepResult :type "HitResult Structure (by ref)"))
  ;[1 1 1] When new farmables are getting placed, checg again to set sprinkler to true
  (if (`self.Is_On`)
    (`self.Set is watered by sprinkler in sprinkler radius` true)))

(event `Switch On/Of Sprinkler`
  ;[1 1 1] Check if the sprinkler is on. If so, turn of.
  ; If trying to turn on, check first if the sprinkler has water. If not, don't do anything.
  ;
  ; The "has water" can be used for things like a storage of water, or is it connected to an automated system, is there water in the pipes or whatever implementation you desire
  (`/Engine/EditorBlueprintResources/ActorMacros.Switch Has Authority` :!label _label
    (:`Authority`
      (if (`self.Is_On`)
        (set `self.Is_On` false)
        ;;[1 1 1] Check all in radius to switch is watered by this sprinkler
        (`self.Set is watered by sprinkler in sprinkler radius` false)
        (elif (`self.Has_Water`)
          (set `self.Is_On` true)
          (`self.Set is watered by sprinkler in sprinkler radius` true))))))

(event `/Game/FarmingSystem/Blueprints/BPI_Farming.Interact`
  (goto _label))

(event `Destroy`
  ;[1 1 1] If destroy, set is watered by sprinkler to false so the reference gets removed by linked farming masters
  (`self.Set is watered by sprinkler in sprinkler radius` false))

(fn `Get GUID`
  (returns (Output_Get :type String))
  ;[1 1 1] Stores the GUID if GUID is empty
  (if (> (`KismetStringLibrary.Len` (`self.GUID`)) 0)
    (return (`self.GUID`))
    (else
      (bind _output_get (set `self.GUID` (`KismetGuidLibrary.Conv_GuidToString` (`KismetGuidLibrary.NewGuid`))))
      (return _output_get))))

(fn `OnRep_Is_On`
  (if (`self.Is_On`)
    (`ActorComponent.SetActive` (`self.Audio`) true false)
    (`ActorComponent.SetActive` (`self.ParticleSystem`) true false)
    (else
      (`ActorComponent.SetActive` (`self.ParticleSystem`) false false)
      (`ActorComponent.SetActive` (`self.Audio`) false false))))

(fn `Set is watered by sprinkler in sprinkler radius`
  (params (`Is watered by sprinkler` :type Boolean))
  (for _array_element (`PrimitiveComponent.GetOverlappingActors` (`self.Sphere`) "/Game/FarmingSystem/Blueprints/Masters/BP_Farming_Master.BP_Farming_Master_C")
    (bind _asbp_farming_master (cast `/Game/FarmingSystem/Blueprints/Masters/BP_Farming_Master` _array_element))
    (if `Is watered by sprinkler`
      (`/Game/FarmingSystem/Blueprints/Masters/BP_Farming_Master.Add Active sprinkler` _asbp_farming_master self)
      (else
        (`/Game/FarmingSystem/Blueprints/Masters/BP_Farming_Master.Remove Active sprinkler` _asbp_farming_master self))))
  (return))

(fn `UserConstructionScript`)