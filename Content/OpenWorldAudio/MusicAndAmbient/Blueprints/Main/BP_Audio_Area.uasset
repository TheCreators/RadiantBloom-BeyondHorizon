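; Trigger volume actor that defines a prioritized music and ambient audio area for the open-world audio system.
; On player overlap it registers with BP_Audio_Manager and takes over the audio if no area is active or its priority is higher, unless the area name already matches.
; End overlap unregisters it from the manager.
; The construction script colors an editor visualization mesh and label by priority, with manager-driven or per-area visibility.
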(event `NewAudioManager`
  (params (AudioReference :type "/Game/OpenWorldAudio/MusicAndAmbient/Blueprints/Main/BP_Audio_Manager Object Reference"))
  ;[0 0.6147 1] Begin Play
  (set `self.AudioReference` AudioReference))

(event `self.ReceiveBeginPlay`
  ;[0 0.6147 1] Begin Play
  (set `self.GameStarted` true)
  (if (`self.Delete_SM_VisualizeArea`)
    (`ActorComponent.K2_DestroyComponent` (`self.SM_VisualizeArea`)))
  (bind _outactors (`GameplayStatics.GetAllActorsOfClass` "/Game/OpenWorldAudio/MusicAndAmbient/Blueprints/Main/BP_Audio_Manager.BP_Audio_Manager_C"))
  (bind _output (`|GetArrayItem` _outactors))
  (`/Engine/EditorBlueprintResources/StandardMacros.IsValid` _output :!label _label
    (:`Is Valid`
      (set `self.AudioReference` _output))
    (:`Is Not Valid`
      (`KismetSystemLibrary.Delay` 0.2)
      (goto _label))))

(event `self.Trigger_Collision.OnComponentBeginOverlap`
  (params (OverlappedComponent :type "PrimitiveComponent Object Reference") (OtherActor :type "Actor Object Reference") (OtherComp :type "PrimitiveComponent Object Reference") (OtherBodyIndex :type Integer) (bFromSweep :type Boolean) (SweepResult :type "HitResult Structure (by ref)"))
  (bind _audioreference (`self.AudioReference`))
  (bind _audioreference_2 (`self.AudioReference`))
  ;[0.9837 1 0.2344] On overlap. Communicate audio area information to the Audio Manager.
  (if (== OtherActor (`GameplayStatics.GetPlayerCharacter` 0))
    (`/Engine/EditorBlueprintResources/StandardMacros.IsValid` _audioreference
      (:`Is Valid`
        (if (`/Game/OpenWorldAudio/MusicAndAmbient/Blueprints/Main/BP_Audio_Manager.StartCompleted` _audioreference)
          (if (== (`KismetArrayLibrary.Array_Find` (`/Game/OpenWorldAudio/MusicAndAmbient/Blueprints/Main/BP_Audio_Manager.OverlappingAudioAreas` (`self.AudioReference`)) self) -1)
            (`/Game/OpenWorldAudio/MusicAndAmbient/Blueprints/Main/BP_Audio_Manager.AddToAudioArray` (`self.AudioReference`) self)
            (if (not (== (`/Game/OpenWorldAudio/MusicAndAmbient/Blueprints/Main/BP_Audio_Manager.AreaName` _audioreference) (`self.AreaName`)))
              (bind _mostrelevantaudioarea (`/Game/OpenWorldAudio/MusicAndAmbient/Blueprints/Main/BP_Audio_Manager.MostRelevantAudioArea` (`self.AudioReference`))
                (:`then`
                  (if (> (`self.Priority`) (`/Game/OpenWorldAudio/MusicAndAmbient/Blueprints/Main/BP_Audio_Area.Priority` _mostrelevantaudioarea))
                    (set `/Game/OpenWorldAudio/MusicAndAmbient/Blueprints/Main/BP_Audio_Manager.MostRelevantAudioArea` self _audioreference_2 :!label _label_2)
                    (`/Game/OpenWorldAudio/MusicAndAmbient/Blueprints/Main/BP_Audio_Manager.SetAudioVariables` _audioreference_2 self)
                    (`/Game/OpenWorldAudio/MusicAndAmbient/Blueprints/Main/BP_Audio_Manager.ChangeAudio` _audioreference_2)))
                (:`else`
                  (goto _label_2))))))))))

(event `self.Trigger_Collision.OnComponentEndOverlap`
  (params (OverlappedComponent :type "PrimitiveComponent Object Reference") (OtherActor :type "Actor Object Reference") (OtherComp :type "PrimitiveComponent Object Reference") (OtherBodyIndex :type Integer))
  ;[0.3632 1 0.3245] End Overlap. Remove this audio area from the Audio Manager.
  (if (== OtherActor (`GameplayStatics.GetPlayerCharacter` 0))
    (bind _audioreference (`self.AudioReference`)
      (:`then`
        (`/Game/OpenWorldAudio/MusicAndAmbient/Blueprints/Main/BP_Audio_Manager.RemoveFromArray` _audioreference self))
      (:`else`))))

(fn `UserConstructionScript`
  (bind _t_priority (`self.T_Priority`))
  ;[0.6406 1 0] Set text variables. (That show priority)
  (`TextRenderComponent.SetTextRenderColor` _t_priority (select `int` (`self.Priority`) :`0` (make `Color` 255 0 0 255) :`1` (make `Color` 255 255 0 255) :`2` (make `Color` 0 255 255 255) :`3` (make `Color` 0 255 0 255) :!type "Color Structure"))
  (`TextRenderComponent.K2_SetText` _t_priority (`KismetTextLibrary.Conv_StringToText` (`KismetStringLibrary.Conv_IntToString` (`self.Priority`))))
  ;[0 0.7656 1] Set visualization and billboard worldscale.
  (`SceneComponent.SetWorldScale3D` (`self.T_Priority`) (1.0 1.0 1.0))
  (`SceneComponent.SetWorldScale3D` (`self.AudioBillboard`) (1.0 1.0 1.0))
  ;[0.9219 1 0] Visualization area visibility and color settings
  (`PrimitiveComponent.SetMaterial` (`self.SM_VisualizeArea`) 0 (select `int` (`self.Priority`) :`0` "/Game/OpenWorldAudio/MusicAndAmbient/Materials/MI_VisualizeARea_0.MI_VisualizeARea_0" :`1` "/Game/OpenWorldAudio/MusicAndAmbient/Materials/MI_VisualizeARea_1.MI_VisualizeARea_1" :`2` "/Game/OpenWorldAudio/MusicAndAmbient/Materials/MI_VisualizeARea_2.MI_VisualizeARea_2" :`3` "/Game/OpenWorldAudio/MusicAndAmbient/Materials/MI_VisualizeARea_3.MI_VisualizeARea_3" :`4` "/Game/OpenWorldAudio/MusicAndAmbient/Materials/MI_VisualizeARea_4.MI_VisualizeARea_4" :`5` "/Game/OpenWorldAudio/MusicAndAmbient/Materials/MI_VisualizeARea_5.MI_VisualizeARea_5" :!type "MaterialInterface Object Reference"))
  (if (`self.bOverwriteVisualizationSettings`)
    (`SceneComponent.SetVisibility` (`self.SM_VisualizeArea`) (`self.bVisualizeArea`) false)
    (else
      (bind _outactors (`GameplayStatics.GetAllActorsOfClass` "/Game/OpenWorldAudio/MusicAndAmbient/Blueprints/Main/BP_Audio_Manager.BP_Audio_Manager_C"))
      (`SceneComponent.SetVisibility` (`self.SM_VisualizeArea`) (`/Game/OpenWorldAudio/MusicAndAmbient/Blueprints/Main/BP_Audio_Manager.bShowAudioVisualizers` (`|GetArrayItem` _outactors)) false))))

(fn `VisualizeArea`
  (params (bNewVisibility :type Boolean))
  (bind _output_get (set `self.bVisualizeArea` bNewVisibility))
  (`SceneComponent.SetVisibility` (`self.SM_VisualizeArea`) _output_get false))