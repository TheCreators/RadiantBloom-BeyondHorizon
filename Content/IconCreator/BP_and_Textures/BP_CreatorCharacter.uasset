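; BP_CreatorCharacter is the icon creator's character Blueprint, but none of its graph logic runs.
; Its mouse wheel, overlap, tick and construction entry points are empty.
; Disconnected nodes would zoom the IconCreatorReference scene capture by changing its FOV and mirror that value to the UI.
; Another orphaned call would save location, rotation and zoom through UIRef, passing the left-right location for the up value too.
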(event `InputAxisKey|MouseWheelAxis`
  (params (AxisValue :type "Float (single-precision)"))
  ;[1 1 1] Zoom in and out
)

(fn `UserConstructionScript`)