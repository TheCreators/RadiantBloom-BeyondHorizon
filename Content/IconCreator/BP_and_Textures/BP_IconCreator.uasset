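; Icon studio actor that frames a skeletal mesh, static mesh or child-actor Blueprint for a SceneCapture2D with adjustable lighting.
; Construction applies meshes, transforms, FOV and light intensities, and fills the capture's show-only list.
; BeginPlay registers level actors by display name in the "IconData" BP_SaveData slot.
; Save stores each item's transform and tagged directional light intensities; Load restores only the transform, as its light-reading branch is disconnected.
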(event `self.ReceiveBeginPlay`
  (bind _returnvalue (`GameplayStatics.DoesSaveGameExist` "IconData"))
  (if _returnvalue
    (bind _returnvalue_2 (`GameplayStatics.LoadGameFromSlot` "IconData"))
    (bind _asbp_save_data (cast `/Game/IconCreator/BP_and_Textures/BP_SaveData` _returnvalue_2))
    (set `self.SaveFile` _asbp_save_data)
    (else
      (bind _returnvalue_3 (`GameplayStatics.CreateSaveGameObject` "/Game/IconCreator/BP_and_Textures/BP_SaveData.BP_SaveData_C"))
      (set `self.SaveFile` _returnvalue_3)))
  (bind _outactors (`GameplayStatics.GetAllActorsOfClass` "/Script/Engine.SkeletalMeshActor"))
  (for _array_element _outactors
    (for _array_element_2 (`/Game/IconCreator/BP_and_Textures/BP_SaveData.ItemData` (`self.SaveFile`))
      (if (`KismetStringLibrary.EqualEqual_StrStr` (`.Name_2_C153390343FAB4F30100FCA445F5F783` (break `/Game/IconCreator/BP_and_Textures/Struct_IconData` _array_element_2)) (`KismetSystemLibrary.GetDisplayName` _array_element))
        (`|ExecutionSequence`
          (:`then_0`
            (break))
          (:`then_1`
            (set `self.Consists` true)))))
    (if (`self.Consists`)
      (set `self.Consists` false)
      (else
        (`KismetArrayLibrary.Array_Add` (`/Game/IconCreator/BP_and_Textures/BP_SaveData.ItemData` (`self.SaveFile`)) (make `/Game/IconCreator/BP_and_Textures/Struct_IconData` (`KismetSystemLibrary.GetDisplayName` _array_element) (1.0 1.0 1.0) (struct) (0.0 0.0 0.0) 0.0 2.0 2.0 2.0 2.0 false 1.0 1.0 0.0 0.0 0.0 0.0 0.0 1.0))
        (`GameplayStatics.SaveGameToSlot` (`self.SaveFile`) "IconData"))))
  (bind _outactors_2 (`GameplayStatics.GetAllActorsOfClass` "/Script/Engine.StaticMeshActor"))
  (for _array_element_3 _outactors_2
    (for _array_element_4 (`/Game/IconCreator/BP_and_Textures/BP_SaveData.ItemData` (`self.SaveFile`))
      (if (`KismetStringLibrary.EqualEqual_StrStr` (`.Name_2_C153390343FAB4F30100FCA445F5F783` (break `/Game/IconCreator/BP_and_Textures/Struct_IconData` _array_element_4)) (`KismetSystemLibrary.GetDisplayName` _array_element_3))
        (`|ExecutionSequence`
          (:`then_0`
            (break))
          (:`then_1`
            (set `self.Consists` true)))))
    (if (`self.Consists`)
      (set `self.Consists` false)
      (else
        (`KismetArrayLibrary.Array_Add` (`/Game/IconCreator/BP_and_Textures/BP_SaveData.ItemData` (`self.SaveFile`)) (make `/Game/IconCreator/BP_and_Textures/Struct_IconData` (`KismetSystemLibrary.GetDisplayName` _array_element_3) (1.0 1.0 1.0) (struct) (0.0 0.0 0.0) 0.0 2.0 2.0 2.0 2.0 false 1.0 1.0 0.0 0.0 0.0 0.0 0.0 1.0))
        (`GameplayStatics.SaveGameToSlot` (`self.SaveFile`) "IconData"))))
  (bind _outactors_3 (`GameplayStatics.GetAllActorsOfClass` "/Script/Engine.Actor"))
  (for _array_element_5 _outactors_3
    (for _array_element_6 (`/Game/IconCreator/BP_and_Textures/BP_SaveData.ItemData` (`self.SaveFile`))
      (if (`KismetStringLibrary.EqualEqual_StrStr` (`.Name_2_C153390343FAB4F30100FCA445F5F783` (break `/Game/IconCreator/BP_and_Textures/Struct_IconData` _array_element_6)) (`KismetSystemLibrary.GetDisplayName` _array_element_5))
        (`|ExecutionSequence`
          (:`then_0`
            (break))
          (:`then_1`
            (set `self.Consists` true)))))
    (if (`self.Consists`)
      (set `self.Consists` false)
      (else
        (`KismetArrayLibrary.Array_Add` (`/Game/IconCreator/BP_and_Textures/BP_SaveData.ItemData` (`self.SaveFile`)) (make `/Game/IconCreator/BP_and_Textures/Struct_IconData` (`KismetSystemLibrary.GetDisplayName` _array_element_5) (1.0 1.0 1.0) (struct) (0.0 0.0 0.0) 0.0 2.0 2.0 2.0 2.0 false 1.0 1.0 0.0 0.0 0.0 0.0 0.0 1.0))
        (`GameplayStatics.SaveGameToSlot` (`self.SaveFile`) "IconData")))))

(event `AddToShowOnlyList`
  (bind _childactor (`ChildActorComponent.ChildActor` (`self.ChildActor`)))
  (`/Engine/EditorBlueprintResources/StandardMacros.IsValid` _childactor
    (:`Is Valid`
      (`KismetArrayLibrary.Array_Add` (`SceneCaptureComponent.ShowOnlyActors` (`self.SceneCaptureComponent2D`)) _childactor)
      (for _array_element (`self.K2_GetComponentsByClass` _childactor "/Script/Engine.SkeletalMeshComponent")
        (`SkeletalMeshComponent.Stop` _array_element)))))

(fn `Load`
  (params (Name :type String) (MeshType :type "/Game/IconCreator/BP_and_Textures/Enums/E_MeshType Enum" :default "NewEnumerator3"))
  (locals (TempMeshType :type "/Game/IconCreator/BP_and_Textures/Enums/E_MeshType Enum" :default "NewEnumerator3"))
  (bind _tempmeshtype (`local.TempMeshType`))
  (if (`self.SaveEnabled`)
    (set `local.TempMeshType` MeshType)
    (bind _returnvalue (`GameplayStatics.LoadGameFromSlot` "IconData"))
    (bind _asbp_save_data (cast `/Game/IconCreator/BP_and_Textures/BP_SaveData` _returnvalue))
    (for _array_element (`/Game/IconCreator/BP_and_Textures/BP_SaveData.ItemData` _asbp_save_data)
      (bind (_name _scale _rotation _location _animpos _light1 _light2 _light3 _light4) (break `/Game/IconCreator/BP_and_Textures/Struct_IconData` _array_element))
      (if (`KismetStringLibrary.EqualEqual_StrStr` _name Name)
        (`|ExecutionSequence`
          (:`then_0`
            (break))
          (:`then_1`
            (`SceneComponent.SetWorldScale3D` (select `/Game/IconCreator/BP_and_Textures/Enums/E_MeshType` _tempmeshtype :`NewEnumerator0` (`self.StaticMesh`) :`NewEnumerator1` (`self.SkeletalMesh`) :`NewEnumerator2` (`self.ChildActor`) :!type "SceneComponent Object Reference") _scale)
            (`SceneComponent.K2_SetRelativeRotation` (select `/Game/IconCreator/BP_and_Textures/Enums/E_MeshType` _tempmeshtype :`NewEnumerator0` (`self.StaticMesh`) :`NewEnumerator1` (`self.SkeletalMesh`) :`NewEnumerator2` (`self.ChildActor`) :!type "SceneComponent Object Reference") _rotation false false)
            (`SceneComponent.K2_SetWorldLocation` (select `/Game/IconCreator/BP_and_Textures/Enums/E_MeshType` _tempmeshtype :`NewEnumerator0` (`self.StaticMesh`) :`NewEnumerator1` (`self.SkeletalMesh`) :`NewEnumerator2` (`self.ChildActor`) :!type "SceneComponent Object Reference") _location false false)))))))

(fn `Save`
  (params (Name :type String) (Meshtype :type "/Game/IconCreator/BP_and_Textures/Enums/E_MeshType Enum" :default "NewEnumerator3"))
  (if (`self.SaveEnabled`)
    (`|ExecutionSequence`
      (:`then_0`
        (bind _outactors (`GameplayStatics.GetAllActorsOfClass` "/Script/Engine.DirectionalLight"))
        (for _array_element _outactors
          (bind _lightcomponent (`Light.LightComponent` _array_element))
          (if (`ActorComponent.ComponentHasTag` _lightcomponent "Light1")
            (bind _intensity (`LightComponentBase.Intensity` _lightcomponent))
            (set `self.Light1` _intensity)
            (elif (`ActorComponent.ComponentHasTag` _lightcomponent "Light2")
              (set `self.Light2` _intensity)
              (elif (`ActorComponent.ComponentHasTag` _lightcomponent "Light3")
                (bind _intensity_2 (`LightComponentBase.Intensity` _lightcomponent))
                (set `self.Light3` _intensity_2)
                (elif (`ActorComponent.ComponentHasTag` _lightcomponent "Light4")
                  (set `self.Light4` _intensity_2)))))))
      (:`then_1`
        (for (_array_element_2 _array_index) (`/Game/IconCreator/BP_and_Textures/BP_SaveData.ItemData` (`self.SaveFile`))
          (if (`KismetStringLibrary.EqualEqual_StrStr` (`.Name_2_C153390343FAB4F30100FCA445F5F783` (break `/Game/IconCreator/BP_and_Textures/Struct_IconData` _array_element_2)) Name)
            (`|ExecutionSequence`
              (:`then_0`
                (break))
              (:`then_1`
                (bind _structout (setmembers `/Game/IconCreator/BP_and_Textures/Struct_IconData` :`StructRef` _array_element_2 :`Scale` (select `/Game/IconCreator/BP_and_Textures/Enums/E_MeshType` Meshtype :`NewEnumerator3` (1.0 1.0 1.0) :`NewEnumerator0` (`SceneComponent.RelativeScale3D` (`self.StaticMesh`)) :`NewEnumerator1` (`SceneComponent.RelativeScale3D` (`self.SkeletalMesh`)) :`NewEnumerator2` (`SceneComponent.RelativeScale3D` (`self.ChildActor`))) :`Rotation` (select `/Game/IconCreator/BP_and_Textures/Enums/E_MeshType` Meshtype :`NewEnumerator0` (`SceneComponent.RelativeRotation` (`self.StaticMesh`)) :`NewEnumerator1` (`SceneComponent.RelativeRotation` (`self.SkeletalMesh`)) :`NewEnumerator2` (`SceneComponent.RelativeRotation` (`self.ChildActor`))) :`Location` (select `/Game/IconCreator/BP_and_Textures/Enums/E_MeshType` Meshtype :`NewEnumerator0` (`SceneComponent.RelativeLocation` (`self.StaticMesh`)) :`NewEnumerator1` (`SceneComponent.K2_GetComponentLocation` (`self.SkeletalMesh`)) :`NewEnumerator2` (`SceneComponent.RelativeLocation` (`self.ChildActor`))) :`AnimPos` 0.0 :`Light1` (`self.Light1`) :`Light2` (`self.Light2`) :`Light3` (`self.Light3`) :`Light4` (`self.Light4`) :`BorderActive` false :`BorderScaleX` 0.0 :`BorderSacleY` 0.0 :`BorderPosX` 0.0 :`BorderPosY` 0.0 :`Background_R` 0.0 :`Background_G` 0.0 :`Background_B` 0.0 :`Background_A` 1.0))
                (`KismetArrayLibrary.Array_Set` (`/Game/IconCreator/BP_and_Textures/BP_SaveData.ItemData` (`self.SaveFile`)) _array_index _structout)
                (`GameplayStatics.SaveGameToSlot` (`self.SaveFile`) "IconData")))))))))

(fn `UserConstructionScript`
  (bind _scenecapturecomponent2d (`self.SceneCaptureComponent2D`))
  (`SkinnedMeshComponent.SetSkinnedAssetAndUpdate` (`self.SkeletalMesh`) (`self.SkeletalM`) true)
  (`StaticMeshComponent.SetStaticMesh` (`self.StaticMesh`) (`self.StaticM`))
  (set `SceneCaptureComponent2D.FOVAngle` (`self.FieldOfView`) (`self.SceneCaptureComponent2D`))
  (`LightComponent.SetIntensity` (`self.ExtraLight1`) (`self.ExtraLight_01`))
  (`LightComponent.SetIntensity` (`self.ExtraLight2`) (`self.ExtraLight_02`))
  (`LightComponent.SetIntensity` (`self.ExtraLight3`) (`self.ExtraLight_03`))
  (`LightComponent.SetIntensity` (`self.ExtraLight4`) (`self.ExtraLight_04`))
  (`LightComponent.SetIntensity` (`self.SpotLight1`) (`self.MainLight1`))
  (`LightComponent.SetIntensity` (`self.SpotLight2`) (`self.MainLight2`))
  (`SceneComponent.K2_SetRelativeTransform` (`self.SkeletalMesh`) (`KismetMathLibrary.MakeTransform` (`self.SkeletalM_Loc`) (`self.SkeletalM_Rot`) (`self.SkeletalM_Scale`)) false false)
  (`SkinnedMeshComponent.SetMinLOD` (`self.SkeletalMesh`) 0)
  (`SceneComponent.K2_SetRelativeTransform` (`self.StaticMesh`) (`KismetMathLibrary.MakeTransform` (`self.StaticM_Loc`) (`self.StaticM_Rot`) (`self.StaticM_Scale`)) false false)
  (bind _outactors (`GameplayStatics.GetAllActorsOfClass` "BP_IconCreator_C"))
  (for _array_element _outactors
    (`KismetArrayLibrary.Array_Add` (`SceneCaptureComponent.ShowOnlyActors` (`self.SceneCaptureComponent2D`)) _array_element)
    (`SceneCaptureComponent.ShowOnlyActorComponents` _scenecapturecomponent2d _array_element))
  (`SceneCaptureComponent.ShowOnlyComponent` _scenecapturecomponent2d (`self.Border`)))