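; Pickup component that makes its owning actor an interactable inventory item, carrying an ItemID row reference and a quantity.
; On BeginPlay it turns on replication for the owner.
; Interacting passes the row name and quantity to the player's BPCInventorySystem and destroys the owner if the add succeeds.
; It always allows interaction, while its outline-mesh and look-at functions return empty results.
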(event `self.ReceiveBeginPlay`
  (`Actor.SetReplicates` (`self.GetOwner`) true))

(event `/Game/InteractionSystem/BPI_Interact.Interact With`
  (params (`Player Character` :type "/Game/ThirdPerson/Blueprints/BP_ThirdPersonCharacter Object Reference"))
  (bind _bpc_inventorysystem (`/Game/ThirdPerson/Blueprints/BP_ThirdPersonCharacter.BPC_InventorySystem` `Player Character`))
  (bind (_item_id_datatable _item_id_rowname) (break `DataTableRowHandle` (`self.Item ID`)))
  (`/Engine/EditorBlueprintResources/StandardMacros.IsValid` _bpc_inventorysystem
    (:`Is Valid`
      (bind _success (`/Game/Inventory/BPC_InventorySystem.Add to Inventory` _bpc_inventorysystem _item_id_rowname (`self.Quantity`)))
      (if _success
        (`Actor.K2_DestroyActor` (`self.GetOwner`))))))

(fn `Can Interact With`
  (returns (`Can Interact` :type Boolean))
  (return true))

(fn `Get Meshes To Outline`
  (returns (Meshes :type "Set of MeshComponent Object Reference"))
  (return))

(fn `Look At`
  (returns (Message :type Text))
  (return ""))