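; BP_Item_Base is the base Blueprint for inventory items in the world that the player can look at and interact with.
; It is always interactable, exposes its Mesh for outlining, returns an empty objective ID, and hands interaction off to its BPCItemData component.
; Its look-at prompt uses that component's ItemID to find a data table row and formats the item's name into pickup text.
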(event `self.ReceiveDestroyed`)

(fn `Can Interact With`
  (returns (`Can Interact` :type Boolean))
  (return true))

(fn `Get Mesh`
  (returns (Mesh :type "StaticMeshComponent Object Reference"))
  (return (`self.Mesh`)))

(fn `Get Meshes To Outline`
  (returns (Meshes :type "Set of MeshComponent Object Reference"))
  (return (`|MakeSet` (`self.Mesh`) :!type "MeshComponent Object Reference")))

(fn `Get Objective ID`
  (returns (ObjectiveID :type String))
  (return ""))

(fn `Interact With`
  (params (`Player Character` :type "/Game/ThirdPerson/Blueprints/BP_ThirdPersonCharacter Object Reference"))
  (`/Game/InteractionSystem/BPI_Interact.Interact With` (`self.BPC_ItemData`) `Player Character`)
  (return))

(fn `Look At`
  (returns (Message :type Text))
  (bind (_item_id_datatable _item_id_rowname) (break `DataTableRowHandle` (`/Game/Inventory/BPC_ItemData.Item ID` (`self.BPC_ItemData`))))
  (bind _returnvalue (`|GetDataTableRow` _item_id_datatable _item_id_rowname)
    (:`then`
      (return (`|FormatText` "Pick up {item}" (`.Name_2_DE6E9AC644375873FE4909B1010CB18F` (break `/Game/Inventory/S_Item` _returnvalue)))))))

(fn `UserConstructionScript`)