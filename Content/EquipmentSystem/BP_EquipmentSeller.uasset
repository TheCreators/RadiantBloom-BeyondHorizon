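; BP_EquipmentSeller is an interactable NPC that opens the equipment shop on the player's HUD when interacted with.
; On BeginPlay it makes its hair, body, head, legs, arms and hat meshes follow the main Mesh through leader pose, forming a modular character.
; It is always interactable, shows a "Buy Equipment" prompt, returns those parts for outlining, and has an empty objective ID.
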(event `self.ReceiveBeginPlay`
  (`self.Assign Parts`))

(event `/Game/InteractionSystem/BPI_Interact.Interact With`
  (params (`Player Character` :type "/Game/ThirdPerson/Blueprints/BP_ThirdPersonCharacter Object Reference"))
  (`/Game/UI/WB_HUD.Display Equipment Shop` (`/Game/ThirdPerson/Blueprints/BP_ThirdPersonCharacter.HUD Widget` `Player Character`)))

(fn `Assign Parts`
  (for _array_element (`|MakeArray` (`self.Hair`) (`self.Body`) (`self.Head`) (`self.Legs`) (`self.Arms`) (`self.Hat`) :!type "SkinnedMeshComponent Object Reference")
    (`SkinnedMeshComponent.SetLeaderPoseComponent` _array_element (`self.Mesh`) false false)))

(fn `Can Interact With`
  (returns (`Can Interact` :type Boolean))
  (return true))

(fn `Get Meshes To Outline`
  (returns (Meshes :type "Set of MeshComponent Object Reference"))
  (return (`|MakeSet` (`self.Hat`) (`self.Hair`) (`self.Body`) (`self.Head`) (`self.Legs`) (`self.Arms`) :!type "MeshComponent Object Reference")))

(fn `Get Objective ID`
  (returns (ObjectiveID :type String))
  (return ""))

(fn `Look At`
  (returns (Message :type Text))
  (return "Buy Equipment"))

(fn `UserConstructionScript`)