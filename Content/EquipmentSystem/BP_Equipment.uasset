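; BP_Equipment is a world pickup actor for an equipment item defined by a data table row.
; Its construction script sets the static mesh from that row.
; It supplies that mesh for outlining and a "Pick up" prompt with the item's name when looked at.
; On interaction, it passes its item data to the player's equipment system component and destroys itself.
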(event `/Game/InteractionSystem/BPI_Interact.Interact With`
  (params (`Player Character` :type "/Game/ThirdPerson/Blueprints/BP_ThirdPersonCharacter Object Reference"))
  (`/Game/EquipmentSystem/BPC_EquipmentSystem.Add Equipment` (`/Game/ThirdPerson/Blueprints/BP_ThirdPersonCharacter.BPC_EquipmentSystem` `Player Character`) (`self.ItemData`))
  (`self.K2_DestroyActor`))

(fn `Get Meshes To Outline`
  (returns (Meshes :type "Set of MeshComponent Object Reference"))
  (return (`|MakeSet` (`self.StaticMesh`) :!type "MeshComponent Object Reference")))

(fn `Look At`
  (returns (Message :type Text))
  (bind _itemdata (`self.ItemData`))
  (bind _returnvalue (`|GetDataTableRow` (break `DataTableRowHandle` (break `/Game/EquipmentSystem/S_Slot` _itemdata)) (`.RowName` (break `DataTableRowHandle` (break `/Game/EquipmentSystem/S_Slot` _itemdata))))
    (:`then`
      (return (`|FormatText` "Pick up {item}" (`KismetTextLibrary.Conv_StringToText` (`.Name_2_0AC983F24260B287AE5B939434214470` (break `/Game/EquipmentSystem/S_Equipment` _returnvalue))))))))

(fn `UserConstructionScript`
  (bind _itemdata (`self.ItemData`))
  (bind _returnvalue (`|GetDataTableRow` (break `DataTableRowHandle` (break `/Game/EquipmentSystem/S_Slot` _itemdata)) (`.RowName` (break `DataTableRowHandle` (break `/Game/EquipmentSystem/S_Slot` _itemdata))))
    (:`then`
      (`StaticMeshComponent.SetStaticMesh` (`self.StaticMesh`) (`.StaticMesh_15_5C89F9894524FD65E0C2AB80BD91FA43` (break `/Game/EquipmentSystem/S_Equipment` _returnvalue))))))