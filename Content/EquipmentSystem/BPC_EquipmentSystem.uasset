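; Player character component that manages owned equipment and the equipped weapon and armor.
; Equip and unequip calls resolve data table rows, update the character and broadcast equipment changes; getters expose equipped items and weapon socket positions.
; Equipment state loads from the game instance on BeginPlay and saves back through it.
; Input toggles a lazily created equipment widget, blocking attacks and movement while open.
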(event `self.ReceiveBeginPlay`
  (bind _asbp_third_person_character (cast `/Game/ThirdPerson/Blueprints/BP_ThirdPersonCharacter` (`self.GetOwner`)))
  (set `self.Player Character BP` _asbp_third_person_character)
  ;[0.5 0 1] Load From Player Economy Save
  (bind _save_game (message `/Game/SaveGame/BPI_SaveGame.Get Game Data` (`GameplayStatics.GetGameInstance`)))
  (`/Engine/EditorBlueprintResources/StandardMacros.IsValid` _save_game
    (:`Is Valid`
      (`self.Load From Player Equipment Save` (`/Game/SaveGame/BP_SaveGame.Player Equipment Save` _save_game))
      (add `self.On Equipment Updated` (`|CreateDelegate` :!event `Save`)))))

(event `EnhancedInput|/Game/ThirdPerson/Input/Actions/IA_OpenEquipment`
  (params (ActionValue :type Boolean) (ElapsedSeconds :type "Float (double-precision)") (TriggeredSeconds :type "Float (double-precision)") (InputAction :type "InputAction Object Reference" :default "/Game/ThirdPerson/Input/Actions/IA_OpenEquipment.IA_OpenEquipment"))
  (bind _returnvalue (`GameplayStatics.GetPlayerController` 0))
  (bind _bpc_attacksystem (`/Game/ThirdPerson/Blueprints/BP_ThirdPersonCharacter.BPC_AttackSystem` (`self.Player Character BP`)))
  (bind _charactermovement (`Character.CharacterMovement` (`self.Player Character BP`)))
  ;[0.8984 1 0] Equipment Widget
  (:`Started`
    (if (not (`self.IsPanelOpened`))
      (set `/Game/Blueprints/BPC_AttackSystem.Can Attack` false _bpc_attacksystem)
      (set `self.IsPanelOpened` true)
      (bind _equipment_widget (`self.Equipment Widget`)
        (:`then`
          (`Widget.SetVisibility` _equipment_widget "Visible"))
        (:`else`
          (bind _returnvalue_2 (`|CreateWidget` "/Game/EquipmentSystem/UI/WB_Equipment.WB_Equipment_C" null self))
          (bind _output_get (set `self.Equipment Widget` _returnvalue_2))
          (`UserWidget.AddToViewport` _output_get 2)
          (`/Game/EquipmentSystem/UI/WB_Equipment.Assign Slots Icons` _output_get (`|MakeArray` (`self.Equiped Weapon`) (`self.Equiped Armor`)))))
      (set `PlayerController.bShowMouseCursor` true _returnvalue)
      (`WidgetBlueprintLibrary.SetInputMode_GameAndUIEx` _returnvalue (`self.Equipment Widget`))
      (`CharacterMovementComponent.SetMovementMode` _charactermovement "MOVE_None" 0)
      (else
        (set `/Game/Blueprints/BPC_AttackSystem.Can Attack` true _bpc_attacksystem :!label _label)
        (set `self.IsPanelOpened` false)
        (bind _equipment_widget_2 (`self.Equipment Widget`)
          (:`then`
            (`Widget.SetVisibility` _equipment_widget_2 "Hidden")
            (set `PlayerController.bShowMouseCursor` false _returnvalue)
            (`WidgetBlueprintLibrary.SetInputMode_GameOnly` _returnvalue)
            (`CharacterMovementComponent.SetMovementMode` _charactermovement "MOVE_Walking" 0))
          (:`else`))))))

(event `EnhancedInput|/Game/ThirdPerson/Input/Actions/IA_CloseUI`
  (params (ActionValue :type Boolean) (ElapsedSeconds :type "Float (double-precision)") (TriggeredSeconds :type "Float (double-precision)") (InputAction :type "InputAction Object Reference" :default "/Game/ThirdPerson/Input/Actions/IA_CloseUI.IA_CloseUI"))
  ;[0.8984 1 0] Equipment Widget
  (:`Started`
    (goto _label)))

(event `Save`
  ;[0 0.8359 1] Saving
  (message `/Game/SaveGame/BPI_SaveGame.Save Player Equipment` (`GameplayStatics.GetGameInstance`) (`self.Get Player Equipment Save`) false))

(fn `Add Equipment`
  (params (`New Item` :type "/Game/EquipmentSystem/S_Slot Structure (by ref)"))
  (`KismetArrayLibrary.Array_AddUnique` (`self.EquipmentSlots`) `New Item`)
  (`self.On Equipment Updated`))

(fn `Equip Item`
  (params (`Item To Equip` :type "/Game/EquipmentSystem/S_Slot Structure"))
  (locals (`Local Equiped Equipment` :type "/Game/EquipmentSystem/S_Equipment Structure"))
  (bind (_local_equiped_equipment_name _local_equiped_equipment_damage _local_equiped_equipment_protectionpercent _local_equiped_equipment_requiredlevel _local_equiped_equipment_icon _local_equiped_equipment_staticmesh _local_equiped_equipment_type) (break `/Game/EquipmentSystem/S_Equipment` (`local.Local Equiped Equipment`)))
  (bind _returnvalue (`|GetDataTableRow` (break `DataTableRowHandle` (break `/Game/EquipmentSystem/S_Slot` `Item To Equip`)) (`.RowName` (break `DataTableRowHandle` (break `/Game/EquipmentSystem/S_Slot` `Item To Equip`))))
    (:`then`
      (bind _output_get (set `local.Local Equiped Equipment` _returnvalue))
      (`/Game/ThirdPerson/Blueprints/BP_ThirdPersonCharacter.Equip Item` (`self.Player Character BP`) _output_get)
      (`|ExecutionSequence`
        (:`then_0`
          (switch `/Game/EquipmentSystem/E_EquipmentType` _local_equiped_equipment_type
            (:`NewEnumerator0`
              (set `self.Is Equiped Weapon A Bow` false)
              (set `self.Equiped Weapon` (`local.Item To Equip`) :!label _label))
            (:`NewEnumerator1`
              (set `self.Is Equiped Weapon A Bow` true)
              (goto _label))
            (:`NewEnumerator2`
              (set `self.Equiped Armor` (`local.Item To Equip`)))))
        (:`then_1`
          (`self.On Equipment Updated`))))))

(fn `Get Equiped Armor`
  (returns (Armor :type "/Game/EquipmentSystem/S_Equipment Structure") (`Has Armor` :type Boolean))
  (bind _equiped_armor (`self.Equiped Armor`))
  (`/Engine/EditorBlueprintResources/StandardMacros.IsValid` (break `DataTableRowHandle` (break `/Game/EquipmentSystem/S_Slot` _equiped_armor))
    (:`Is Valid`
      (bind _returnvalue (`|GetDataTableRow` (break `DataTableRowHandle` (break `/Game/EquipmentSystem/S_Slot` _equiped_armor)) (`.RowName` (break `DataTableRowHandle` (break `/Game/EquipmentSystem/S_Slot` _equiped_armor))))
        (:`then`
          (return _returnvalue true))
        (:`RowNotFound`
          _)))
    (:`Is Not Valid`
      _))
  (return (struct) false))

(fn `Get Equiped Weapon`
  (returns (Weapon :type "/Game/EquipmentSystem/S_Equipment Structure") (`Has Weapon` :type Boolean))
  (bind _equiped_weapon (`self.Equiped Weapon`))
  (`/Engine/EditorBlueprintResources/StandardMacros.IsValid` (break `DataTableRowHandle` (break `/Game/EquipmentSystem/S_Slot` _equiped_weapon))
    (:`Is Valid`
      (bind _returnvalue (`|GetDataTableRow` (break `DataTableRowHandle` (break `/Game/EquipmentSystem/S_Slot` _equiped_weapon)) (`.RowName` (break `DataTableRowHandle` (break `/Game/EquipmentSystem/S_Slot` _equiped_weapon))))
        (:`then`
          (return _returnvalue true))
        (:`RowNotFound`
          _)))
    (:`Is Not Valid`
      _))
  (return (struct) false))

(fn `Get Equiped Weapon Start And End Positions`
  (returns (`Has Weapon` :type Boolean) (Start :type "Vector Structure") (End :type "Vector Structure"))
  (locals (`Local Start Socket` :type Name) (`Local End Socket` :type Name) (`Local Weapon` :type String))
  (bind (_weapon _has_weapon) (`self.Get Equiped Weapon`))
  (bind _equipment_weapon (`/Game/ThirdPerson/Blueprints/BP_ThirdPersonCharacter.Equipment Weapon` (`self.Player Character BP`)))
  (set `local.Local Weapon` (break `/Game/EquipmentSystem/S_Equipment` _weapon))
  (set `local.Local Start Socket` (`.StartSocket_24_F722CB534A77EF4ED93253AB9F12C220` (break `/Game/EquipmentSystem/S_Equipment` _weapon)))
  (set `local.Local End Socket` (`.EndSocket_26_31C02E8B45845255E821E3A16C2B91A9` (break `/Game/EquipmentSystem/S_Equipment` _weapon)))
  (if (or _has_weapon (`|EnumInequality` (`.Type_18_67EF1DD34A03BC763486F38A9B67222F` (break `/Game/EquipmentSystem/S_Equipment` _weapon)) "NewEnumerator0"))
    (`|ExecutionSequence`
      (:`then_0`
        (if (not (`SceneComponent.DoesSocketExist` _equipment_weapon (`local.Local End Socket`)))
          (`KismetSystemLibrary.PrintText` (`|FormatText` "End Socket \"{Socket}\" of weapon \"{Weapon}\" is missing!" (`local.Local End Socket`) (`local.Local Weapon`)) true true (struct :`G` 0.66 :`B` 1.0 :`A` 1.0) 5.0)))
      (:`then_1`
        (if (not (`SceneComponent.DoesSocketExist` _equipment_weapon (`local.Local Start Socket`)))
          (`KismetSystemLibrary.PrintText` (`|FormatText` "Start Socket \"{Socket}\" of weapon \"{Weapon}\" is missing!" (`local.Local Start Socket`) (`local.Local Weapon`)) true true (struct :`G` 0.66 :`B` 1.0 :`A` 1.0) 5.0)))
      (:`then_2`
        (return true (`SceneComponent.GetSocketLocation` _equipment_weapon (`local.Local Start Socket`)) (`SceneComponent.GetSocketLocation` _equipment_weapon (`local.Local End Socket`)))))
    (else
      (return false (0.0 0.0 0.0) (0.0 0.0 0.0)))))

(fn `Get Player Equipment Save`
  (returns (`Player Equipment Save` :type "/Game/SaveGame/S_PlayerEquipmentSave Structure"))
  (return (make `/Game/SaveGame/S_PlayerEquipmentSave` (`self.EquipmentSlots`) (`self.Equiped Weapon`) (`self.Equiped Armor`))))

(fn `Load From Player Equipment Save`
  (params (`Player Equipment Save` :type "/Game/SaveGame/S_PlayerEquipmentSave Structure"))
  (bind ((`EquipedWeapon_10_3756970B45C78FFBC1A0A6973C80CDEE` _equipedweapon)) (break `/Game/SaveGame/S_PlayerEquipmentSave` (`local.Player Equipment Save`)))
  (bind ((`EquipedArmor_11_8682A9B94738DA22424B59AFED12C157` _equipedarmor)) (break `/Game/SaveGame/S_PlayerEquipmentSave` (`local.Player Equipment Save`)))
  (bind _item_datatable (break `DataTableRowHandle` (break `/Game/EquipmentSystem/S_Slot` _equipedarmor)))
  (bind _item_datatable_2 (break `DataTableRowHandle` (break `/Game/EquipmentSystem/S_Slot` _equipedweapon)))
  (`|ExecutionSequence`
    (:`then_0`
      (set `self.EquipmentSlots` (`.EquipmentSlots_5_43CCEE85460F4909E893BA951AD562EA` (break `/Game/SaveGame/S_PlayerEquipmentSave` (`local.Player Equipment Save`)))))
    (:`then_1`
      (`/Engine/EditorBlueprintResources/StandardMacros.IsValid` _item_datatable_2
        (:`Is Valid`
          (`self.Equip Item` _equipedweapon))))
    (:`then_2`
      (`/Engine/EditorBlueprintResources/StandardMacros.IsValid` _item_datatable
        (:`Is Valid`
          (`self.Equip Item` _equipedarmor))))))

(fn `Unequip Item`
  (params (`Equipment Type` :type "/Game/EquipmentSystem/E_EquipmentType Enum" :default "NewEnumerator0"))
  (`/Game/ThirdPerson/Blueprints/BP_ThirdPersonCharacter.Unequip Item` (`self.Player Character BP`) `Equipment Type`)
  (`|ExecutionSequence`
    (:`then_0`
      (switch `/Game/EquipmentSystem/E_EquipmentType` (`local.Equipment Type`)
        (:`NewEnumerator0`
          (set `self.Equiped Weapon` (struct) :!label _label))
        (:`NewEnumerator1`
          (goto _label))
        (:`NewEnumerator2`
          (set `self.Equiped Armor` (struct)))))
    (:`then_1`
      (`self.On Equipment Updated`))))