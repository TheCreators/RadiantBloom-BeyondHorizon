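; Arrow projectile actor that resolves damage, effects and cleanup when its mesh hits something.
; On hit it stops the Niagara trail, destroys itself if it struck its instigator, and otherwise sphere-traces at HitPoint.
; A successful trace damages the hit actor, hides the mesh, plays hit effects and optional explosion sound, removes flames, then destroys after a short delay.
; A failed trace disables collision, plays a wall-hit sound and delays destruction longer.
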(event `self.StaticMesh.OnComponentHit`
  (params (HitComponent :type "PrimitiveComponent Object Reference") (OtherActor :type "Actor Object Reference") (OtherComp :type "PrimitiveComponent Object Reference") (NormalImpulse :type "Vector Structure") (Hit :type "HitResult Structure (by ref)"))
  (bind _trailniagara (`self.TrailNiagara`))
  (bind _returnvalue (`SceneComponent.K2_GetComponentLocation` (`self.Hit Point`)))
  (if (not (`self.IsDestroying`))
    (`NiagaraComponent.SetVariableVec3` _trailniagara "BeamEnd" (0.0 0.0 0.0))
    (`NiagaraComponent.SetVariableFloat` _trailniagara "SpawnRate" 0.0)
    (if (!= OtherActor (`self.GetInstigator`))
      (bind (_outhit _returnvalue_2) (`KismetSystemLibrary.SphereTraceSingle` _returnvalue _returnvalue 5.0 "TraceTypeQuery4"))
      (if _returnvalue_2
        (`GameplayStatics.ApplyDamage` OtherActor (`self.Arrow Damage`) (`self.GetInstigatorController`) self)
        (`GameplayStatics.PlaySoundAtLocation` "/Game/Audio/Bow/MS_ArrowHitFlash.MS_ArrowHitFlash" (`self.K2_GetActorLocation`) (struct) 0.1 1.0 0.0 "/Game/Audio/SA_Character.SA_Character" null null null)
        (`SceneComponent.SetVisibility` (`self.StaticMesh`) false false)
        (`ActorComponent.Activate` (`self.HitNiagara`) false)
        (bind _explotionsound (`self.ExplotionSound`)
          (:`then`
            (`GameplayStatics.PlaySoundAtLocation` _explotionsound (`self.K2_GetActorLocation`) (struct) 2.0 1.0 0.0 "/Game/Audio/Bow/SA_ArrowExplotion.SA_ArrowExplotion" null null null))
          (:`else`
            _))
        (bind _flamesniagara (`self.FlamesNiagara`)
          (:`then`
            (`ActorComponent.K2_DestroyComponent` _flamesniagara))
          (:`else`
            _))
        (set `self.IsDestroying` true)
        (`KismetSystemLibrary.Delay` 3.0)
        (`self.K2_DestroyActor`)
        (else
          (`self.SetActorEnableCollision` false)
          (`GameplayStatics.PlaySoundAtLocation` "/Game/Audio/Bow/MS_ArrowHitWall.MS_ArrowHitWall" (`self.K2_GetActorLocation`) (struct) 2.0 1.0 0.0 "/Game/Audio/SA_Character.SA_Character" null null null)
          (`KismetSystemLibrary.Delay` 30.0)
          (`self.K2_DestroyActor`)))
      (else
        (`self.K2_DestroyActor`)))))

(fn `UserConstructionScript`)