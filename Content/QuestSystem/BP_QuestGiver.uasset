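; Quest-giver Blueprint that shows "Ask for Quests" when looked at and offers the player a list of quests.
; Interacting toggles a WB_QuestGiver widget initialized with its Quests array, switching cursor visibility and input mode to match.
; Activating a quest clears the previously active one, flags the new one in the array and passes it to the player character's BPCQuest component.
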(event `/Game/Inventory/BPI_Interact.Interact With`
  (params (`Player Character` :type "/Game/ThirdPerson/Blueprints/BP_ThirdPersonCharacter Object Reference"))
  (bind _returnvalue (`GameplayStatics.GetPlayerController` 0))
  ;[0.05127 0.05127 0.05127] Interaction
  (bind _quests_widget (`self.Quests Widget`)
    (:`then`
      ;;[0.05127 0.05127 0.05127] Setup Inputs
      (set `PlayerController.bShowMouseCursor` false _returnvalue :!label _label)
      (`WidgetBlueprintLibrary.SetInputMode_GameOnly` _returnvalue)
      ;;[0.05127 0.05127 0.05127] UI
      (`Widget.RemoveFromParent` _quests_widget)
      (set `self.Quests Widget` null))
    (:`else`
      (set `PlayerController.bShowMouseCursor` true _returnvalue)
      (`WidgetBlueprintLibrary.SetInputMode_GameAndUIEx` _returnvalue _quests_widget)
      (bind _returnvalue_2 (`|CreateWidget` "/Game/QuestSystem/UI/WB_QuestGiver.WB_QuestGiver_C"))
      (set `self.Quests Widget` _returnvalue_2)
      (`/Game/QuestSystem/UI/WB_QuestGiver.Init` _returnvalue_2 self (`self.Quests`))
      (`UserWidget.AddToViewport` _returnvalue_2 2))))

(event `Close Widget`
  ;[0.05127 0.05127 0.05127] Interaction
  (goto _label))

(event `Set Quest As Active`
  (params (Quest :type "/Game/QuestSystem/S_Quest Structure"))
  (bind _quests (`self.Quests`))
  (`self.Deactivate Active QUEST`)
  (bind _structout (setmembers `/Game/QuestSystem/S_Quest` :`StructRef` (`|GetArrayItem` _quests (`KismetArrayLibrary.Array_Find` _quests Quest)) :`Active` true))
  (set `self.Active Quest` _structout)
  (bind _asbp_third_person_character (cast `/Game/ThirdPerson/Blueprints/BP_ThirdPersonCharacter` (`GameplayStatics.GetPlayerCharacter` 0)))
  (`/Game/QuestSystem/BPC_Quest.Set Active Quest` (`/Game/ThirdPerson/Blueprints/BP_ThirdPersonCharacter.BPC_Quest` _asbp_third_person_character) _structout))

(event `Deactivate Active Quest`
  (bind _quests (`self.Quests`))
  (bind _returnvalue (`KismetArrayLibrary.Array_Find` _quests (`self.Active Quest`)))
  (if (!= _returnvalue -1)
    (setmembers `/Game/QuestSystem/S_Quest` :`StructRef` (`|GetArrayItem` _quests _returnvalue) :`Active` false)
    (bind _asbp_third_person_character (cast `/Game/ThirdPerson/Blueprints/BP_ThirdPersonCharacter` (`GameplayStatics.GetPlayerCharacter` 0)))
    (`/Game/QuestSystem/BPC_Quest.Remove Active Quest` (`/Game/ThirdPerson/Blueprints/BP_ThirdPersonCharacter.BPC_Quest` _asbp_third_person_character))))

(fn `Look At`
  (returns (Message :type Text))
  (return "Ask for Quests"))

(fn `UserConstructionScript`)