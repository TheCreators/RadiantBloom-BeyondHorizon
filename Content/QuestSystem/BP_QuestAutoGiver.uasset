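; BP_QuestAutoGiver is a quest system Blueprint that adds a configured quest to the player's quest log.
; Its GiveQuest event gets the player character's BPCQuestLog and passes the quest's row name to QueryActiveQuest.
; When that query returns true, it calls AddNewQuest with the same row name.
; Nothing in the Blueprint triggers GiveQuest itself, and the construction script is empty.
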(event `GiveQuest`
  (if (`/Game/QuestSystem/BPC_QuestLog.QueryActiveQuest` (`/Game/ThirdPerson/Blueprints/BP_ThirdPersonCharacter.BPC_QuestLog` (`/Game/CommonFunctionLibrary.GetMyPlayerCharacter`)) (`.RowName` (break `DataTableRowHandle` (`self.Quest`))))
    (`/Game/QuestSystem/BPC_QuestLog.AddNewQuest` (`/Game/ThirdPerson/Blueprints/BP_ThirdPersonCharacter.BPC_QuestLog` (`/Game/CommonFunctionLibrary.GetMyPlayerCharacter`)) (`.RowName` (break `DataTableRowHandle` (`self.Quest`))))))

(fn `UserConstructionScript`)