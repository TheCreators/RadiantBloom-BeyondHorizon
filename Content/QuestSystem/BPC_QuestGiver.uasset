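; Quest giver component that offers a quest, referenced by a data table row handle, when its owner is interacted with.
; Its interact function queries the player character's quest log for that row name and prints a notice if the quest is already active.
; Otherwise it looks up the row and prints the quest name as placeholder display, without adding it to the log.
; Either path returns the owner's display name.
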(fn `DisplayQuest`
  (bind (_datatable _rowname) (break `DataTableRowHandle` (`self.Quest`)))
  (bind _returnvalue (`|GetDataTableRow` _datatable _rowname)
    (:`then`
      (`KismetSystemLibrary.PrintText` (`.Name_20_38871AC440F3B7176C3552AB09CAF8DF` (break `/Game/QuestSystem/S_Quest` _returnvalue))))))

(fn `Interact RENAME`
  (returns (ObjectiveID :type String))
  (bind _returnvalue (`KismetSystemLibrary.GetDisplayName` (`self.GetOwner`)))
  (if (`/Game/QuestSystem/BPC_QuestLog.QueryActiveQuest` (`/Game/ThirdPerson/Blueprints/BP_ThirdPersonCharacter.BPC_QuestLog` (`/Game/CommonFunctionLibrary.GetMyPlayerCharacter`)) (`.RowName` (break `DataTableRowHandle` (`self.Quest`))))
    (`KismetSystemLibrary.PrintString` "Aleady on Quest")
    (return _returnvalue)
    (else
      (`self.DisplayQuest`)
      (return _returnvalue))))