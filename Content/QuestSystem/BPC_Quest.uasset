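; BPC_Quest is a quest component that tracks the active quest and shows it on the HUD.
; Setting a quest stores it, lazily creates a WB_ActiveQuestHUD widget on the viewport if none is valid, and passes the quest to that widget.
; Removing the active quest clears the reference, takes the widget off screen and releases it.
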(event `Set Active Quest`
  (params (Quest :type "/Game/QuestSystem/S_Quest Structure"))
  (set `self.Active Quest` Quest)
  (`self.Active Quest HUD Widget`
    (:`then`
      _)
    (:`else`
      (bind _returnvalue (`|CreateWidget` "/Game/QuestSystem/UI/WB_ActiveQuestHUD.WB_ActiveQuestHUD_C"))
      (bind _output_get (set `self.Active Quest HUD Widget` _returnvalue))
      (`UserWidget.AddToViewport` _output_get 0)))
  (`/Game/QuestSystem/UI/WB_ActiveQuestHUD.Set Quest` _output_get (`self.Active Quest`)))

(event `Remove Active Quest`
  (set `self.Active Quest` (struct))
  (bind _active_quest_hud_widget (`self.Active Quest HUD Widget`)
    (:`then`
      (`Widget.RemoveFromParent` _active_quest_hud_widget)
      (set `self.Active Quest HUD Widget` null))
    (:`else`)))