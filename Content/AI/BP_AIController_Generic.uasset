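; Generic AI controller that runs BT_AI and turns sight and hearing perception into blackboard data for chasing and investigating.
; Each perception update feeds both SIghtDetection, which sets or clears Target Actor, and HearingDetection, which records the stimulus location as Inestigation Location.
; Hearing also triggers InvestigationIcon on the controlled BP_AI pawn.
; Any non-sight stimulus, including hearing, also clears Target Actor.
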(event `self.ReceiveBeginPlay`
  (`self.RunBehaviorTree` "/Game/AI/BT_AI.BT_AI"))

(event `self.AIPerception.OnTargetPerceptionUpdated`
  (params (Actor :type "Actor Object Reference") (Stimulus :type "AIStimulus Structure"))
  ;[0.05127 0.05127 0.05127] Detect and Chase / Investiagte Target
  (`self.SIght Detection` Actor Stimulus)
  (`self.Hearing Detection` Actor Stimulus))

(fn `Hearing Detection`
  (params (Actor :type "Actor Object Reference") (Stimulus :type "AIStimulus Structure"))
  (bind _returnvalue (`AIPerceptionSystem.GetSenseClassForStimulus` Stimulus))
  (if (== _returnvalue "/Script/AIModule.AISense_Hearing")
    (`BlackboardComponent.SetValueAsVector` (`AIBlueprintHelperLibrary.GetBlackboard` null) "Inestigation Location" (`.StimulusLocation` (break `AIStimulus` Stimulus)))
    (bind _asbp_ai (cast `/Game/AI/BP_AI` (`self.K2_GetPawn`)))
    (`/Game/AI/BP_AI.Investigation Icon` _asbp_ai)))

(fn `SIght Detection`
  (params (Actor :type "Actor Object Reference") (Stimulus :type "AIStimulus Structure"))
  (bind _returnvalue (`AIBlueprintHelperLibrary.GetBlackboard` null))
  (bind _returnvalue_2 (`AIPerceptionSystem.GetSenseClassForStimulus` Stimulus))
  (if (== _returnvalue_2 "/Script/AIModule.AISense_Sight")
    (if (`.bSuccessfullySensed` (break `AIStimulus` Stimulus))
      (`BlackboardComponent.SetValueAsObject` _returnvalue "Target Actor" Actor)
      (else
        (`BlackboardComponent.SetValueAsObject` _returnvalue "Target Actor" null :!label _label)))
    (else
      (goto _label))))

(fn `UserConstructionScript`)