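; Modular skeleton enemy character that builds a randomized appearance in its construction script, leaving BeginPlay to its parent.
; Body-part meshes follow the inherited Mesh through leader pose, while hand static meshes attach to its sockets.
; Equipment flags drive clothing-fit morph targets across all skeletal parts.
; Helmet, boots, chest armour and gloves are then picked at random, each with an empty option, along with the chest mesh's skin material.
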(event `self.ReceiveBeginPlay`
  (`parent.ReceiveBeginPlay`))

(fn `GetMorphTargetValue`
  (params (CanMorph :type Boolean))
  (returns (ReturnValue :type "Float (double-precision)"))
  (return (`KismetMathLibrary.SelectFloat` 1.0 0.0 CanMorph)))

(fn `IsDefaultMeshInheritungItsAnimationAsset`
  (returns (ReturnValue :type Boolean))
  (bind _mesh (`self.Mesh`))
  (if (`|EnumEquality` (`SkeletalMeshComponent.GetAnimationMode` _mesh) "AnimationSingleNode")
    (`/Engine/EditorBlueprintResources/StandardMacros.IsValid` (`.AnimToPlay` (break `SingleAnimationPlayData` (`SkeletalMeshComponent.AnimationData` _mesh)))
      (:`Is Valid`
        (return true)))))

(fn `Randomize Clothes and Skin`
  (set `SkeletalMeshComponent.SkeletalMeshAsset` (`KismetArrayLibrary.Array_Random` (`|MakeArray` null "/Game/Characters/Skeleton/CharacterParts_Skeleton/Meshes/Skeleton/Helm/SK_ma_tal_nrw_skeleton_helmet_01_a.SK_ma_tal_nrw_skeleton_helmet_01_a" "/Game/Characters/Skeleton/CharacterParts_Skeleton/Meshes/Skeleton/Helm/SK_ma_tal_nrw_skeleton_helmet_01_b.SK_ma_tal_nrw_skeleton_helmet_01_b" :!type "SkeletalMesh Object Reference")) (`self.SK_Hat`))
  (set `SkeletalMeshComponent.SkeletalMeshAsset` (`KismetArrayLibrary.Array_Random` (`|MakeArray` null "/Game/Characters/Skeleton/CharacterParts_Skeleton/Meshes/Skeleton/Boots/SK_ma_tal_nrw_skeleton_shoe_01.SK_ma_tal_nrw_skeleton_shoe_01" "/Game/Characters/Skeleton/CharacterParts_Skeleton/Meshes/Skeleton/Boots/SK_ma_tal_nrw_skeleton_shoe_02.SK_ma_tal_nrw_skeleton_shoe_02" "/Game/Characters/Skeleton/CharacterParts_Skeleton/Meshes/Skeleton/Boots/SK_ma_tal_nrw_skeleton_shoe_03.SK_ma_tal_nrw_skeleton_shoe_03" :!type "SkeletalMesh Object Reference")) (`self.SK_Boots`))
  (set `SkeletalMeshComponent.SkeletalMeshAsset` (`KismetArrayLibrary.Array_Random` (`|MakeArray` null "/Game/Characters/Skeleton/CharacterParts_Skeleton/Meshes/Skeleton/Chest/SK_ma_tal_nrw_skeleton_chest_01.SK_ma_tal_nrw_skeleton_chest_01" "/Game/Characters/Skeleton/CharacterParts_Skeleton/Meshes/Skeleton/Chest/SK_ma_tal_nrw_skeleton_chest_02.SK_ma_tal_nrw_skeleton_chest_02" "/Game/Characters/Skeleton/CharacterParts_Skeleton/Meshes/Skeleton/Chest/SK_ma_tal_nrw_skeleton_chest_03.SK_ma_tal_nrw_skeleton_chest_03" "/Game/Characters/Skeleton/CharacterParts_Skeleton/Meshes/Skeleton/Chest/SK_ma_tal_nrw_skeleton_chest_04.SK_ma_tal_nrw_skeleton_chest_04" "/Game/Characters/Skeleton/CharacterParts_Skeleton/Meshes/Skeleton/Chest/SK_ma_tal_nrw_skeleton_chest_05.SK_ma_tal_nrw_skeleton_chest_05" :!type "SkeletalMesh Object Reference")) (`self.SK_Armour_Extra`))
  (set `SkeletalMeshComponent.SkeletalMeshAsset` (`KismetArrayLibrary.Array_Random` (`|MakeArray` null "/Game/Characters/Skeleton/CharacterParts_Skeleton/Meshes/Skeleton/Bracers_gloves/SK_ma_tal_nrw_skeleton_bracers_01.SK_ma_tal_nrw_skeleton_bracers_01" "/Game/Characters/Skeleton/CharacterParts_Skeleton/Meshes/Skeleton/Bracers_gloves/SK_ma_tal_nrw_skeleton_bracers_02.SK_ma_tal_nrw_skeleton_bracers_02" "/Game/Characters/Skeleton/CharacterParts_Skeleton/Meshes/Skeleton/Bracers_gloves/SK_ma_tal_nrw_skeleton_bracers_03.SK_ma_tal_nrw_skeleton_bracers_03" "/Game/Characters/Skeleton/CharacterParts_Skeleton/Meshes/Skeleton/Bracers_gloves/SK_ma_tal_nrw_skeleton_glove_01.SK_ma_tal_nrw_skeleton_glove_01" :!type "SkeletalMesh Object Reference")) (`self.SK_Hand/Glove`))
  (`PrimitiveComponent.SetMaterial` (`self.SK_Chest`) 0 (`KismetArrayLibrary.Array_Random` (`|MakeArray` "/Game/Characters/Skeleton/CharacterParts_Skeleton/Materials/Skeleton/MI_skeleton_base.MI_skeleton_base" "/Game/Characters/Skeleton/CharacterParts_Skeleton/Materials/Skeleton/MI_skeleton_base_dark.MI_skeleton_base_dark" "/Game/Characters/Skeleton/CharacterParts_Skeleton/Materials/Skeleton/MI_skeleton_base_green.MI_skeleton_base_green" :!type "MaterialInterface Object Reference"))))

(fn `SetMasterPoseComponentForParts`
  ;[0 0 0] Updates all Part components (skeletal and static meshes) to follow the Master Pose of Mesh (Inherited).
  ;
  ; This means, you can set the character's animation in its editor Details Panel or in Mesh (Inherited) component itself, which then gets used for all other Part components as well automatically.
  (`SkinnedMeshComponent.SetLeaderPoseComponent` (`self.SK_Armour_Extra`) (`self.Mesh`) false false)
  (`SkinnedMeshComponent.SetLeaderPoseComponent` (`self.SK_Hand/Glove`) (`self.Mesh`) false false)
  (`SkinnedMeshComponent.SetLeaderPoseComponent` (`self.SK_Chest`) (`self.Mesh`) false false)
  (`SkinnedMeshComponent.SetLeaderPoseComponent` (`self.SK_Head`) (`self.Mesh`) false false)
  (`SkinnedMeshComponent.SetLeaderPoseComponent` (`self.SK_Hair`) (`self.Mesh`) false false)
  (`SkinnedMeshComponent.SetLeaderPoseComponent` (`self.SK_Hat`) (`self.Mesh`) false false)
  (`SkinnedMeshComponent.SetLeaderPoseComponent` (`self.SK_Pants`) (`self.Mesh`) false false)
  (`SkinnedMeshComponent.SetLeaderPoseComponent` (`self.SK_Boots`) (`self.Mesh`) false false)
  (`SkinnedMeshComponent.SetLeaderPoseComponent` (`self.SK_Skin_Extra`) (`self.Mesh`) false false)
  (`SceneComponent.K2_AttachToComponent` (`self.SM_LeftHand`) (`self.Mesh`) "LeftHandSocket" "KeepRelative" "KeepRelative" "KeepRelative" true)
  (`SceneComponent.K2_AttachToComponent` (`self.SM_RightHand`) (`self.Mesh`) "RightHandSocket" "KeepRelative" "KeepRelative" "KeepRelative" true))

(fn `UpdateMorphTargets`
  (bind _array (`|MakeArray` (`self.SK_Hat`) (`self.SK_Hair`) (`self.SK_Head`) (`self.SK_Chest`) (`self.SK_Hand/Glove`) (`self.SK_Armour_Extra`) (`self.SK_Skin_Extra`) (`self.SK_Boots`) (`self.SK_Pants`)))
  (for _array_element _array
    (`SkeletalMeshComponent.SetMorphTarget` _array "hat_equipped" (`self.GetMorphTargetValue` (`self.HatEquipped`)) true)
    (`SkeletalMeshComponent.SetMorphTarget` _array "gloves_equipped" (`self.GetMorphTargetValue` (`self.GlovesEquipped`)) true)
    (`SkeletalMeshComponent.SetMorphTarget` _array_element "hat_equipped" (`self.GetMorphTargetValue` (`self.HatEquipped`)) true)
    (`SkeletalMeshComponent.SetMorphTarget` _array_element "gloves_equipped" (`self.GetMorphTargetValue` (`self.GlovesEquipped`)) true)
    (`SkeletalMeshComponent.SetMorphTarget` _array_element "pants_long_equipped" (`self.GetMorphTargetValue` (`self.boot_medium_equipped`)) true)
    (`SkeletalMeshComponent.SetMorphTarget` _array_element "Collar_high" (`self.GetMorphTargetValue` (`self.collar_high`)) true)
    (`SkeletalMeshComponent.SetMorphTarget` _array_element "Robe_equipped" (`self.GetMorphTargetValue` (`self.Robe_equipped`)) true)
    (`SkeletalMeshComponent.SetMorphTarget` _array_element "boot_medium_equipped" (`self.GetMorphTargetValue` (`self.boot_medium_equipped`)) true)
    (`SkeletalMeshComponent.SetMorphTarget` _array_element "boot_high_equipped" (`self.GetMorphTargetValue` (`self.boot_high_equipped`)) true)))

(fn `UserConstructionScript`
  (set `self.Refresh` false)
  (`self.UpdateMorphTargets`)
  (`self.SetMasterPoseComponentForParts`)
  (`self.Randomize Clothes and Skin`)
  (`parent.UserConstructionScript`))