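; Base villager AI Blueprint that builds a modular civilian with a randomized appearance at BeginPlay.
; AssignParts makes the hat, body, hair, head, arms and legs meshes follow the main Mesh through Leader Pose.
; RandomizeParts then picks a random entry from each part's list, async loads it and applies it to the matching component once loaded.
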(event `self.ReceiveBeginPlay`
  (`self.Assign Parts`)
  (`self.Randomize Parts`)
  (`parent.ReceiveBeginPlay`))

(event `Randomize Parts`
  ;[0 0.5312 1] Randomizing Parts
  (`|ExecutionSequence`
    (:`then_0`
      (bind _object (`|LoadAsset` (`KismetArrayLibrary.Array_Random` (`self.Hats`)))
        (:`Completed`
          (bind _asskeletal_mesh (cast `SkeletalMesh` _object))
          (`SkeletalMeshComponent.SetSkeletalMeshAsset` (`self.Hat Mesh`) _asskeletal_mesh))))
    (:`then_1`
      (bind _object_2 (`|LoadAsset` (`KismetArrayLibrary.Array_Random` (`self.Bodies`)))
        (:`Completed`
          (bind _asskeletal_mesh_2 (cast `SkeletalMesh` _object_2))
          (`SkeletalMeshComponent.SetSkeletalMeshAsset` (`self.Body Mesh`) _asskeletal_mesh_2))))
    (:`then_2`
      (bind _object_3 (`|LoadAsset` (`KismetArrayLibrary.Array_Random` (`self.Hairs`)))
        (:`Completed`
          (bind _asskeletal_mesh_3 (cast `SkeletalMesh` _object_3))
          (`SkeletalMeshComponent.SetSkeletalMeshAsset` (`self.Hair Mesh`) _asskeletal_mesh_3))))
    (:`then_3`
      (bind _object_4 (`|LoadAsset` (`KismetArrayLibrary.Array_Random` (`self.Heads`)))
        (:`Completed`
          (bind _asskeletal_mesh_4 (cast `SkeletalMesh` _object_4))
          (`SkeletalMeshComponent.SetSkeletalMeshAsset` (`self.Head Mesh`) _asskeletal_mesh_4))))
    (:`then_4`
      (bind _object_5 (`|LoadAsset` (`KismetArrayLibrary.Array_Random` (`self.Arms`)))
        (:`Completed`
          (bind _asskeletal_mesh_5 (cast `SkeletalMesh` _object_5))
          (`SkeletalMeshComponent.SetSkeletalMeshAsset` (`self.Arms Mesh`) _asskeletal_mesh_5))))
    (:`then_5`
      (bind _object_6 (`|LoadAsset` (`KismetArrayLibrary.Array_Random` (`self.Legs`)))
        (:`Completed`
          (bind _asskeletal_mesh_6 (cast `SkeletalMesh` _object_6))
          (`SkeletalMeshComponent.SetSkeletalMeshAsset` (`self.Legs Mesh`) _asskeletal_mesh_6))))))

(fn `Assign Parts`
  (for _array_element (`|MakeArray` (`self.Hat Mesh`) (`self.Body Mesh`) (`self.Hair Mesh`) (`self.Head Mesh`) (`self.Arms Mesh`) (`self.Legs Mesh`) :!type "SkinnedMeshComponent Object Reference")
    (`SkinnedMeshComponent.SetLeaderPoseComponent` _array_element (`self.Mesh`) false false)))

(fn `UserConstructionScript`
  (`parent.UserConstructionScript`))