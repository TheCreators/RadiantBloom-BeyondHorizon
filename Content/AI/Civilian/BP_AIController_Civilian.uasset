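; AI controller for civilian NPCs that makes them panic when they sense damage.
; On BeginPlay it runs the civilian behavior tree and sets the Blackboard state to Passive.
; Perception updates are filtered for damage stimuli, which switch any handled state to Panicing with the sensed actor stored as the panic target.
; Panicing briefly resets the state to Passive first, so repeated damage registers as a state change.
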(event `self.ReceiveBeginPlay`
  (`self.RunBehaviorTree` "/Game/AI/Civilian/BT_AI_Civilian.BT_AI_Civilian")
  (`self.Set State As Passive`))

(event `self.AIPerception.OnPerceptionUpdated`
  (params (UpdatedActors :type "Array of Actor Object Reference (by ref)"))
  (for _array_element UpdatedActors
    (bind _sensed (`self.Can Sense Actor` _array_element "NewEnumerator3"))
    (if _sensed
      (`self.Handle Sensed Damage` _array_element))))

(fn `Can Sense Actor`
  (params (Actor :type "Actor Object Reference") (Sense :type "/Game/AI/Enums/E_AISense Enum" :default "NewEnumerator0"))
  (returns (Sensed :type Boolean) (Stimulus :type "AIStimulus Structure"))
  (bind _info (`AIPerceptionComponent.GetActorsPerception` (`self.AIPerception`) Actor))
  (for _array_element (`.LastSensedStimuli` (break `ActorPerceptionBlueprintInfo` _info))
    (bind _returnvalue (`AIPerceptionSystem.GetSenseClassForStimulus` _array_element))
    (if (== _returnvalue (select `/Game/AI/Enums/E_AISense` (`local.Sense`) :`NewEnumerator1` "/Script/AIModule.AISense_Sight" :`NewEnumerator2` "/Script/AIModule.AISense_Hearing" :`NewEnumerator3` "/Script/AIModule.AISense_Damage" :!type "Object Class Reference"))
      (return (`.bSuccessfullySensed` (break `AIStimulus` _array_element)) _array_element))))

(fn `Get Current State`
  (returns (State :type "/Game/AI/Enums/E_AIState Enum"))
  (return (cast `/Game/AI/Enums/E_AIState` (`BlackboardComponent.GetValueAsEnum` (`self.Blackboard`) (`self.State Key Name`)))))

(fn `Handle Sensed Damage`
  (params (Actor :type "Actor Object Reference"))
  (switch `/Game/AI/Enums/E_AIState` (`self.Get Current State`)
    (:`NewEnumerator0`
      _)
    (:`NewEnumerator2`
      _)
    (:`NewEnumerator4`
      _))
  (`self.Set State As Panicing` (`local.Actor`)))

(fn `Set State As Panicing`
  (params (`Panic Target` :type "Actor Object Reference"))
  (`BlackboardComponent.SetValueAsObject` (`self.Blackboard`) (`self.Panic Target Key Name`) `Panic Target`)
  (`self.Set State As Passive`)
  (`BlackboardComponent.SetValueAsEnum` (`self.Blackboard`) (`self.State Key Name`) (enumliteral `/Game/AI/Enums/E_AIState` "NewEnumerator4"))
  (set `self.Panic Target` (`local.Panic Target`)))

(fn `Set State As Passive`
  (`BlackboardComponent.SetValueAsEnum` (`self.Blackboard`) (`self.State Key Name`) (enumliteral `/Game/AI/Enums/E_AIState` "NewEnumerator0")))

(fn `UserConstructionScript`
  (`parent.UserConstructionScript`))