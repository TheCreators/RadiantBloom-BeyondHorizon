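; Player interaction component that shows a prompt for whatever the camera looks at and lets the player interact with it.
; On BeginPlay it caches the third-person character and adds a message widget to the viewport.
; Each tick it sphere-traces along the follow camera's forward vector, storing the hit actor and displaying its LookAtMessage, or clearing both on a miss.
; IA_Interact calls InteractWithMessage on the stored actor, passing the character.
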(event `self.ReceiveBeginPlay`
  ;[0.05127 0.05127 0.05127] Player Character
  (bind _asbp_third_person_character (cast `/Game/ThirdPerson/Blueprints/BP_ThirdPersonCharacter` (`GameplayStatics.GetPlayerCharacter` 0)))
  (set `self.Character BP` _asbp_third_person_character)
  ;[0.05127 0.05127 0.05127] Display Message Widget
  (bind _returnvalue (`|CreateWidget` "/Game/Inventory/UI/WB_DisplayMessage.WB_DisplayMessage_C"))
  (bind _output_get (set `self.Display Message` _returnvalue))
  (`UserWidget.AddToViewport` _output_get 0))

(event `self.ReceiveTick`
  (params (DeltaSeconds :type "Float (single-precision)"))
  (`self.Interaction Trace`))

(event `EnhancedInput|/Game/ThirdPerson/Input/Actions/IA_Interact`
  (params (ActionValue :type Boolean) (ElapsedSeconds :type "Float (double-precision)") (TriggeredSeconds :type "Float (double-precision)") (InputAction :type "InputAction Object Reference" :default "/Game/ThirdPerson/Input/Actions/IA_Interact.IA_Interact"))
  (:`Started`
    (bind _look_at_actor (`self.Look At Actor`)
      (:`then`
        (message `/Game/Inventory/BPI_Interact.Interact With` _look_at_actor (`self.Character BP`)))
      (:`else`))))

(fn `Interaction Trace`
  (bind _followcamera (`/Game/ThirdPerson/Blueprints/BP_ThirdPersonCharacter.FollowCamera` (`self.Character BP`)))
  (bind _returnvalue (`SceneComponent.K2_GetComponentLocation` _followcamera))
  (bind _returnvalue_2 (`KismetMathLibrary.GetForwardVector` (`SceneComponent.K2_GetComponentRotation` _followcamera)))
  (bind (_outhit _returnvalue_3) (`KismetSystemLibrary.SphereTraceSingle` (+ _returnvalue (* _returnvalue_2 (`self.Interation Range Start`))) (+ _returnvalue (* _returnvalue_2 (`self.Interaction Range End`))) 25.0 "TraceTypeQuery3" false (`|MakeArray` (`self.GetOwner`)) "None" true (struct :`R` 1.0 :`A` 1.0) (struct :`G` 1.0 :`A` 1.0) 0.1))
  (if _returnvalue_3
    (bind (_bblockinghit _binitialoverlap _time _distance _location _impactpoint _normal _impactnormal _physmat _hitactor) (`GameplayStatics.BreakHitResult` _outhit))
    (if (!= _hitactor (`self.Look At Actor`))
      (bind _output_get (set `self.Look At Actor` _hitactor))
      (bind _message (message `/Game/Inventory/BPI_Interact.Look At` _output_get))
      (`/Game/Inventory/UI/WB_DisplayMessage.Show Message` (`self.Display Message`) _message))
    (else
      (set `self.Look At Actor` null)
      (`/Game/Inventory/UI/WB_DisplayMessage.Show Message` (`self.Display Message`) ""))))