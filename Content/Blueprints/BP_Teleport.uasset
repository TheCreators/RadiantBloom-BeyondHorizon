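; Trigger-box teleporter that moves the third-person player character between streamed levels.
; On overlap it reports the use_teleport objective, switches off combat music on audio managers through an interface, and requests a save from the game instance.
; It then shows a loading screen, unloads and loads the configured levels, applies the destination location and rotation, and removes the screen.
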(event `self.Box.OnComponentBeginOverlap`
  (params (OverlappedComponent :type "PrimitiveComponent Object Reference") (OtherActor :type "Actor Object Reference") (OtherComp :type "PrimitiveComponent Object Reference") (OtherBodyIndex :type Integer) (bFromSweep :type Boolean) (SweepResult :type "HitResult Structure (by ref)"))
  (bind _asbp_third_person_character (cast `/Game/ThirdPerson/Blueprints/BP_ThirdPersonCharacter` OtherActor))
  (`/Game/ThirdPerson/Blueprints/BP_ThirdPersonCharacter.OnObjectiveIDCalled` _asbp_third_person_character "use_teleport" 1)
  (`|ExecutionSequence`
    (:`then_0`
      (bind _outactors (`GameplayStatics.GetAllActorsWithInterface` "/Game/OpenWorldAudio/MusicAndAmbient/Blueprints/Misc/BPI_AudioManager.BPI_AudioManager_C"))
      (for _array_element _outactors
        (message `/Game/OpenWorldAudio/MusicAndAmbient/Blueprints/Misc/BPI_AudioManager.SetCombatMusic` _array_element false)))
    (:`then_1`
      (message `/Game/Save/BPI_Persistence.RequestSave` (`GameplayStatics.GetGameInstance`) false)
      (bind _returnvalue (`|CreateWidget` "/Game/UI/Menu/LoadingScreen.LoadingScreen_C"))
      (`UserWidget.AddToViewport` _returnvalue 100)
      (`GameplayStatics.UnloadStreamLevelBySoftObjectPtr` (`self.Level To Unload`) true)
      (`GameplayStatics.LoadStreamLevelBySoftObjectPtr` (`self.Level To Load`) true)
      (`self.K2_SetActorLocationAndRotation` _asbp_third_person_character (`self.Location After Teleport`) (`self.Rotation After Teleport`) false false)
      (`Widget.RemoveFromParent` _returnvalue))))

(fn `UserConstructionScript`)