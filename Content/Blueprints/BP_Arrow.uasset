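; Arrow actor that damages what it strikes, using its instigator as the damage source and ignoring that instigator as a target.
; On mesh hit, a small sphere trace at HitPoint on a custom channel separates damageable hits from other surfaces.
; A successful trace applies ArrowDamage, plays a hit sound and destroys the arrow.
; A failed trace disables collision and plays a wall sound, leaving the arrow for a delay before destroying it.
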(event `self.StaticMesh.OnComponentHit`
  (params (HitComponent :type "PrimitiveComponent Object Reference") (OtherActor :type "Actor Object Reference") (OtherComp :type "PrimitiveComponent Object Reference") (NormalImpulse :type "Vector Structure") (Hit :type "HitResult Structure (by ref)"))
  (bind _returnvalue (`SceneComponent.K2_GetComponentLocation` (`self.Hit Point`)))
  (if (!= OtherActor (`self.GetInstigator`))
    (bind (_outhit _returnvalue_2) (`KismetSystemLibrary.SphereTraceSingle` _returnvalue _returnvalue 5.0 "TraceTypeQuery4"))
    (if _returnvalue_2
      (`GameplayStatics.ApplyDamage` OtherActor (`self.Arrow Damage`) (`self.GetInstigatorController`) self)
      (`GameplayStatics.PlaySoundAtLocation` "/Game/Audio/Bow/MS_ArrowHitFlash.MS_ArrowHitFlash" (`self.K2_GetActorLocation`) (struct) 0.1 1.0 0.0 "/Game/Audio/SA_Character.SA_Character" null null null)
      (else
        (`self.SetActorEnableCollision` false)
        (`GameplayStatics.PlaySoundAtLocation` "/Game/Audio/Bow/MS_ArrowHitWall.MS_ArrowHitWall" (`self.K2_GetActorLocation`) (struct) 2.0 1.0 0.0 "/Game/Audio/SA_Character.SA_Character" null null null)
        (`KismetSystemLibrary.Delay` 30.0))))
  (`self.K2_DestroyActor`))

(fn `UserConstructionScript`)