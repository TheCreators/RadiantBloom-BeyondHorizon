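; BP_Dummy is an enemy character that takes hits, can be stealth-assassinated from behind, and drops loot on death.
; Damage plays a random hit montage, launches it along the player's facing and lowers health through a stats component, ragdolling it when depleted.
; StealthBackAssasin plays the paired victim montage, returns an alignment transform to the caller, then triggers delayed death.
; Health bar and proximity-shown assassinate widgets rotate toward the camera every tick.
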(event `self.ReceiveBeginPlay`
  ;[0.05127 0.05127 0.05127] Init
  (bind _aswb_in_game_health_bar (cast `/Game/UI/WB_InGameHealthBar` (`WidgetComponent.GetWidget` (`self.Health Bar Widget`))))
  (bind _output_get (set `self.Health Bar UI` _aswb_in_game_health_bar))
  (`/Game/UI/WB_InGameHealthBar.Set To Enemy` _output_get)
  (add `/Game/Blueprints/BPC_PlayerStats.On Health Changed` (`self.BPC_PlayerStats`) (`|CreateDelegate` (`self.Health Bar UI`) :!event `Update Health`)))

(event `Die From Assasin`
  ;[0.05127 0.05127 0.05127] Assassination Ragdoll
  (`|ExecutionSequence`
    (:`then_0`
      (`KismetSystemLibrary.Delay` 2.5)
      (`self.Die` true))
    (:`then_1`
      (`KismetSystemLibrary.Delay` 1.4)
      (`GameplayStatics.PlaySoundAtLocation` "/Game/Audio/Grunts/SC_MaleDeath.SC_MaleDeath" (`self.K2_GetActorLocation`) (struct) 1.0 1.0 0.0 null null null null))))

(event `self.Assassination Radius.OnComponentBeginOverlap`
  (params (OverlappedComponent :type "PrimitiveComponent Object Reference") (OtherActor :type "Actor Object Reference") (OtherComp :type "PrimitiveComponent Object Reference") (OtherBodyIndex :type Integer) (bFromSweep :type Boolean) (SweepResult :type "HitResult Structure (by ref)"))
  ;[0.05127 0.05127 0.05127] Head Widgets
  (cast `/Game/ThirdPerson/Blueprints/BP_ThirdPersonCharacter` OtherActor)
  (`SceneComponent.SetVisibility` (`self.Assasinate Widget`) true false))

(event `self.Assassination Radius.OnComponentEndOverlap`
  (params (OverlappedComponent :type "PrimitiveComponent Object Reference") (OtherActor :type "Actor Object Reference") (OtherComp :type "PrimitiveComponent Object Reference") (OtherBodyIndex :type Integer))
  ;[0.05127 0.05127 0.05127] Head Widgets
  (cast `/Game/ThirdPerson/Blueprints/BP_ThirdPersonCharacter` OtherActor)
  (`SceneComponent.SetVisibility` (`self.Assasinate Widget`) false false))

(event `self.ReceiveTick`
  (params (DeltaSeconds :type "Float (single-precision)"))
  ;[0.05127 0.05127 0.05127] Head Widgets
  (`SceneComponent.K2_SetWorldRotation` (`self.Assasinate Widget`) (`KismetMathLibrary.FindLookAtRotation` (`SceneComponent.K2_GetComponentLocation` (`self.Health Bar Widget`)) (`SceneComponent.K2_GetComponentLocation` (`PlayerCameraManager.TransformComponent` (`GameplayStatics.GetPlayerCameraManager` 0)))) false false)
  (`SceneComponent.K2_SetWorldRotation` (`self.Health Bar Widget`) (`KismetMathLibrary.FindLookAtRotation` (`SceneComponent.K2_GetComponentLocation` (`self.Health Bar Widget`)) (`SceneComponent.K2_GetComponentLocation` (`PlayerCameraManager.TransformComponent` (`GameplayStatics.GetPlayerCameraManager` 0)))) false false))

(event `self.ReceiveAnyDamage`
  (params (Damage :type "Float (single-precision)") (DamageType :type "DamageType Object Reference") (InstigatedBy :type "Controller Object Reference") (DamageCauser :type "Actor Object Reference"))
  ;[0.05127 0.05127 0.05127] Taking Damage
  (`self.PlayAnimMontage` (`|GetArrayItem` (`self.Hit Aims`) (`KismetMathLibrary.RandomIntegerInRange` 0 (- (`KismetArrayLibrary.Array_Length` (`self.Hit Aims`)) 1))))
  (bind _asbp_third_person_character (cast `/Game/ThirdPerson/Blueprints/BP_ThirdPersonCharacter` (`GameplayStatics.GetPlayerCharacter` 0)))
  (`self.LaunchCharacter` (* (`KismetMathLibrary.GetForwardVector` (`self.K2_GetActorRotation` _asbp_third_person_character)) 700.0))
  (`GameplayStatics.PlaySoundAtLocation` "/Game/Audio/Grunts/MaleDeath2.MaleDeath2" (`self.K2_GetActorLocation`) (struct) 1.0 (`KismetMathLibrary.RandomFloatInRange` 0.8 1.2) 0.0 "/Game/Audio/SA_Character.SA_Character" null null null)
  (bind _is_player_dead (`/Game/Blueprints/BPC_PlayerStats.Decrease Health` (`self.BPC_PlayerStats`) Damage))
  (if _is_player_dead
    (`self.Die` false)))

(event `Destroy`
  (params (Delay :type "Float (double-precision)"))
  ;[0.05127 0.05127 0.05127] Destory
  (`KismetSystemLibrary.Delay` Delay)
  (`self.K2_DestroyActor`))

(fn `Die`
  (params (Mute :type Boolean))
  (if (not Mute)
    (`GameplayStatics.PlaySoundAtLocation` "/Game/Audio/Grunts/SC_MaleDeath.SC_MaleDeath" (`self.K2_GetActorLocation`) (struct) 1.0 1.0 0.0 null null null null))
  (`PrimitiveComponent.SetSimulatePhysics` (`self.Mesh`) true)
  (`self.Hide Widgets`)
  (`/Game/LootDropSystem/BPC_LootDropSystem.Drop Loot` (`self.BPC_LootDrop`))
  (`self.Destroy` 1.0))

(fn `Hide Widgets`
  (`SceneComponent.SetVisibility` (`self.Health Bar Widget`) false false)
  (`SceneComponent.SetVisibility` (`self.Assasinate Widget`) false false))

(fn `Stealth Back Assasin`
  (returns (`REF Location` :type "Vector Structure") (`Assasin Rotation` :type "Rotator Structure"))
  (`self.Hide Widgets`)
  (`self.PlayAnimMontage` "/Game/Characters/RPG_Character/Animations/Assassinations/Paired_Knife_Stealth_KidneyAndNeck_Vic_Montage.Paired_Knife_Stealth_KidneyAndNeck_Vic_Montage")
  (`self.Die From Assasin`)
  (return (`SceneComponent.K2_GetComponentLocation` (`self.Assasin REF`)) (`self.K2_GetActorRotation`)))

(fn `UserConstructionScript`)