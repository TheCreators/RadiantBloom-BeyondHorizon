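; BP_Chest is an interactable chest that opens its inventory in the player's HUD container view.
; Interaction passes its BPCInventorySystem component to the player's HUD widget, and the same component handles saving its contents to the save game.
; It always allows interaction, outlines its static mesh, shows "Open Chest" when looked at, and reports the "openchest" objective ID.
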(event `/Game/InteractionSystem/BPI_Interact.Interact With`
  (params (`Player Character` :type "/Game/ThirdPerson/Blueprints/BP_ThirdPersonCharacter Object Reference"))
  (`/Game/UI/WB_HUD.Show Container` (`/Game/ThirdPerson/Blueprints/BP_ThirdPersonCharacter.HUD Widget` `Player Character`) (`self.BPC_InventorySystem`)))

(event `/Game/Save/BPI_Saveable.SaveData`
  (params (SaveGameRef :type "/Game/Save/BP_SaveGame Object Reference"))
  ;[0 0.0625 1] Save
  (`/Game/Inventory/BPC_InventorySystem.SaveData` (`self.BPC_InventorySystem`) SaveGameRef))

(fn `Can Interact With`
  (returns (`Can Interact` :type Boolean))
  (return true))

(fn `Get Meshes To Outline`
  (returns (Meshes :type "Set of MeshComponent Object Reference"))
  (return (`|MakeSet` (`self.StaticMesh`) :!type "MeshComponent Object Reference")))

(fn `Get Objective ID`
  (returns (ObjectiveID :type String))
  (return "openchest"))

(fn `Look At`
  (returns (Message :type Text))
  (return "Open Chest"))

(fn `UserConstructionScript`)