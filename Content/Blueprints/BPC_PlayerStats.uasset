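; Player stats component that tracks health, stamina, XP and level for the third-person character.
; Health and stamina functions adjust values, cap gains at the max and broadcast change events, while the decrease functions return whether the stat is depleted.
; XP and level write directly to the character's HUD widget.
; Reaching max XP adds a level, raises the next threshold, discards overflow XP and plays level-up sounds.
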(event `self.ReceiveBeginPlay`
  ;[0.05127 0.05127 0.05127] Get Character BP
  (bind _asbp_third_person_character (cast `/Game/ThirdPerson/Blueprints/BP_ThirdPersonCharacter` (`GameplayStatics.GetPlayerCharacter` 0)))
  (set `self.Player Character BP` _asbp_third_person_character)
  (`KismetSystemLibrary.DelayUntilNextTick`)
  (`self.On Health Changed` (`self.Health`) (`self.Max Health`))
  (`self.On Stamina Changed` (`self.Stamina`) (`self.Max Stamina`))
  ;[0.05127 0.05127 0.05127] Init Level
  (`TextBlock.SetText` (`/Game/UI/WB_HUD.LevelText` (`/Game/ThirdPerson/Blueprints/BP_ThirdPersonCharacter.HUD Widget` (`self.Player Character BP`))) (`KismetTextLibrary.Conv_IntToText` (`self.Level`))))

(fn `Decrease Health`
  (params (Amount :type "Float (double-precision)"))
  (returns (`Is Player Dead` :type Boolean))
  (if (> (`self.Health`) 0.0)
    (set `self.Health` (- (`self.Health`) Amount))
    (`self.On Health Changed` (`self.Health`) (`self.Max Health`))
    (if (<= (`self.Health`) 0.0)
      (set `self.Is Dead` true :!label _label)
      (else
        (set `self.Is Dead` false)))
    (else
      (goto _label)))
  (return (`self.Is Dead`)))

(fn `Decrease Stamina`
  (params (Amount :type "Float (double-precision)"))
  (returns (`No Stamina Left` :type Boolean))
  (if (> (`self.Stamina`) 0.0)
    (set `self.Stamina` (- (`self.Stamina`) Amount))
    (`self.On Stamina Changed` (`self.Stamina`) (`self.Max Stamina`))
    (if (<= (`self.Stamina`) 0.0)
      _
      (else
        (return false))))
  (return true))

(fn `Increase Health`
  (params (Amount :type "Float (double-precision)"))
  (set `self.Health` (+ (`self.Health`) Amount))
  (if (> (`self.Health`) (`self.Max Health`))
    (set `self.Health` (`self.Max Health`)))
  (`self.On Health Changed` (`self.Health`) (`self.Max Health`)))

(fn `Increase Level`
  (params (Amount :type Integer))
  (set `self.Level` (+ (`self.Level`) Amount))
  (set `self.Max XP` (+ (`self.Max XP`) 150.0))
  (set `self.XP` 0.0)
  (`TextBlock.SetText` (`/Game/UI/WB_HUD.LevelText` (`/Game/ThirdPerson/Blueprints/BP_ThirdPersonCharacter.HUD Widget` (`self.Player Character BP`))) (`KismetTextLibrary.Conv_IntToText` (`self.Level`)))
  (`GameplayStatics.PlaySound2D` "/Game/Audio/UI/LevelUp1.LevelUp1" 1.0 1.0 0.0 null null)
  (`GameplayStatics.PlaySound2D` "/Game/Audio/UI/LevelUp2.LevelUp2" 1.0 1.0 0.0 null null))

(fn `Increase Max Health`
  (params (Amount :type "Float (double-precision)"))
  (set `self.Max Health` (+ (`self.Max Health`) Amount))
  (`self.On Health Changed` (`self.Health`) (`self.Max Health`)))

(fn `Increase Max Stamina`
  (params (Amount :type "Float (double-precision)"))
  (set `self.Max Stamina` (+ (`self.Max Stamina`) Amount))
  (`self.On Stamina Changed` (`self.Stamina`) (`self.Max Stamina`)))

(fn `Increase Stamina`
  (params (Amount :type "Float (double-precision)"))
  (set `self.Stamina` (+ (`self.Stamina`) Amount))
  (if (> (`self.Stamina`) (`self.Max Stamina`))
    (set `self.Stamina` (`self.Max Stamina`)))
  (`self.On Stamina Changed` (`self.Stamina`) (`self.Max Stamina`)))

(fn `Increase XP`
  (params (Amount :type "Float (double-precision)"))
  (set `self.XP` (+ (`self.XP`) Amount))
  (if (>= (`self.XP`) (`self.Max XP`))
    (`self.Increase Level` 1))
  (`ProgressBar.SetPercent` (`/Game/UI/WB_HUD.XPBar` (`/Game/ThirdPerson/Blueprints/BP_ThirdPersonCharacter.HUD Widget` (`self.Player Character BP`))) (/ (`self.XP`) (`self.Max XP`)))
  (`TextBlock.SetText` (`/Game/UI/WB_HUD.XPText` (`/Game/ThirdPerson/Blueprints/BP_ThirdPersonCharacter.HUD Widget` (`self.Player Character BP`))) (`|FormatText` "{Current XP} / {Max XP}" (`self.XP`) (`self.Max XP`))))

(fn `Set Health`
  (params (Health :type "Float (double-precision)"))
  (set `self.Health` Health)
  (if (> (`self.Health`) (`self.Max Health`))
    (set `self.Health` (`self.Max Health`)))
  (`self.On Health Changed` (`self.Health`) (`self.Max Health`)))