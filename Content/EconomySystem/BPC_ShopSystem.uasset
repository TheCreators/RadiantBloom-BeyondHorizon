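; Shop component that lets the player buy and sell single items for coins.
; It caches the player's BP_ThirdPersonCharacter on BeginPlay and works through its economy and inventory components.
; Buy checks funds and removes coins only after the item is added; Sell takes one item from a slot found in reverse search and adds coins.
; Successful trades report buy_ or sell_ prefixed item IDs as objective progress.
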(event `self.ReceiveBeginPlay`
  ;[0.05127 0.05127 0.05127] Init
  (bind _asbp_third_person_character (cast `/Game/ThirdPerson/Blueprints/BP_ThirdPersonCharacter` (`GameplayStatics.GetPlayerCharacter` 0)))
  (set `self.Character BP` _asbp_third_person_character))

(fn `Buy`
  (params (`Item ID` :type Name) (`Buy Price` :type Integer))
  (bind _bpc_inventorysystem (`/Game/ThirdPerson/Blueprints/BP_ThirdPersonCharacter.BPC_InventorySystem` (`self.Character BP`)))
  (bind _enough (`/Game/EconomySystem/BPC_EconomySystem.Has Enough Coins` (`/Game/ThirdPerson/Blueprints/BP_ThirdPersonCharacter.BPC_EconomySystem` (`self.Character BP`)) (`local.Buy Price`)))
  (if _enough
    (bind _success (`/Game/Inventory/BPC_InventorySystem.Add to Inventory` _bpc_inventorysystem (`local.Item ID`) 1))
    (if _success
      (`/Game/Inventory/BPC_InventorySystem.MC Update` _bpc_inventorysystem)
      (`/Game/EconomySystem/BPC_EconomySystem.Remove Coins` (`/Game/ThirdPerson/Blueprints/BP_ThirdPersonCharacter.BPC_EconomySystem` (`self.Character BP`)) (`local.Buy Price`))
      (`/Game/ThirdPerson/Blueprints/BP_ThirdPersonCharacter.OnObjectiveIDCalled` (`/Game/CommonFunctionLibrary.GetMyPlayerCharacter`) (`KismetTextLibrary.Conv_TextToString` (`|FormatText` "buy_{name}" (`local.Item ID`))) 1))))

(fn `Sell`
  (params (`Item ID` :type Name) (`Sell Price` :type Integer))
  (bind _bpc_inventorysystem (`/Game/ThirdPerson/Blueprints/BP_ThirdPersonCharacter.BPC_InventorySystem` (`self.Character BP`)))
  (if (`/Game/Inventory/BPC_InventorySystem.Query Inventory` (`/Game/ThirdPerson/Blueprints/BP_ThirdPersonCharacter.BPC_InventorySystem` (`self.Character BP`)) (`local.Item ID`) 1)
    (bind (_index _found_slot) (`/Game/Inventory/BPC_InventorySystem.Find Slot` _bpc_inventorysystem (`local.Item ID`) true false))
    (if _found_slot
      (`/Game/Inventory/BPC_InventorySystem.Remove from Inventory` _bpc_inventorysystem _index false true)
      (`/Game/Inventory/BPC_InventorySystem.MC Update` _bpc_inventorysystem)
      (`/Game/EconomySystem/BPC_EconomySystem.Add Coins` (`/Game/ThirdPerson/Blueprints/BP_ThirdPersonCharacter.BPC_EconomySystem` (`self.Character BP`)) (`local.Sell Price`))
      (`/Game/ThirdPerson/Blueprints/BP_ThirdPersonCharacter.OnObjectiveIDCalled` (`/Game/CommonFunctionLibrary.GetMyPlayerCharacter`) (`KismetTextLibrary.Conv_TextToString` (`|FormatText` "sell_{name}" (`local.Item ID`))) 1))))