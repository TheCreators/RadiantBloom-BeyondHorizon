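; Economy component that tracks the owner's coin balance and saves it with the game.
; Add, remove and set functions change the balance and broadcast OnCoinsChanged; removal fails and returns false when funds are short.
; On BeginPlay it requests a load from the GameInstance, then broadcasts the balance a tick later.
; Save and load events write and read the coins through the save object's player economy struct.
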(event `self.ReceiveBeginPlay`
  ;[0.8984 0 1] Request Load
  (message `/Game/Save/BPI_Persistence.RequestLoad` (`GameplayStatics.GetGameInstance`) self)
  (`KismetSystemLibrary.DelayUntilNextTick`)
  (`self.On Coins Changed` (`self.Coins`)))

(event `/Game/Save/BPI_Saveable.SaveData`
  (params (SaveGameRef :type "/Game/Save/BP_SaveGame Object Reference"))
  ;[0 1 0.8828] Save
  (set `/Game/Save/BP_SaveGame.PlayerEconomySaveData` (make `/Game/Save/Structures/S_PlayerEconomySaveData` (`self.Coins`)) SaveGameRef))

(event `/Game/Save/BPI_Saveable.LoadData`
  (params (SaveGameRef :type "/Game/Save/BP_SaveGame Object Reference"))
  ;[0 1 0.8828] Save
  (`self.Set Coins` (`.Coins_3_D90AE9904646718275553DAB23E73053` (break `/Game/Save/Structures/S_PlayerEconomySaveData` (`/Game/Save/BP_SaveGame.PlayerEconomySaveData` SaveGameRef)))))

(fn `Add Coins`
  (params (Amount :type Integer))
  (bind _output_get (set `self.Coins` (+ Amount (`self.Coins`))))
  (`self.On Coins Changed` _output_get))

(fn `Has Enough Coins`
  (params (Amount :type Integer))
  (returns (Enough :type Boolean))
  (return (<= Amount (`self.Coins`))))

(fn `Remove Coins`
  (params (Amount :type Integer))
  (returns (Success :type Boolean))
  (bind _returnvalue (- (`self.Coins`) Amount))
  (if (>= _returnvalue 0)
    (bind _output_get (set `self.Coins` _returnvalue))
    (`self.On Coins Changed` _output_get)
    (return true)
    (else
      (return false))))

(fn `Set Coins`
  (params (Amount :type Integer))
  (bind _output_get (set `self.Coins` Amount))
  (`self.On Coins Changed` _output_get))